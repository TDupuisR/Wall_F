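; Laser beam actor that traces along its up vector and passes hits to BPI_LightBeams actors, supporting bounced beam chains.
; Each tick a thin box trace sizes the beam mesh, three rect lights and box audio attenuation to the blocking hit or max range.
; Interface messages start, update or release the next beam as the hit actor changes, and release it on destruction.
; BeginPlay tints the mesh's dynamic material and lights with the beam color.
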(event `self.ReceiveBeginPlay`
  (bind _lightslist (`self.LightsList`))
  (`KismetArrayLibrary.Array_Clear` _lightslist)
  (`KismetArrayLibrary.Array_Add` _lightslist (`self.RectLight-D`))
  (`KismetArrayLibrary.Array_Add` _lightslist (`self.RectLight-UL`))
  (`KismetArrayLibrary.Array_Add` _lightslist (`self.RectLight-UR`))
  (`self.Set Color`)
  (add `self.OnDestroyed` (delegate `OnDestroyed_Event`)))

(event `OnDestroyed_Event` :!signature `self.OnDestroyed`
  (params (DestroyedActor :type "Actor Object Reference"))
  (bind _lasthitactor (`self.LastHitActor`))
  (if (`KismetSystemLibrary.DoesImplementInterface` _lasthitactor "/Game/WallFContent/BluePrint/EnvironmentInteractives/Laser/BPI_LightBeams.BPI_LightBeams_C")
    (message `/Game/WallFContent/BluePrint/EnvironmentInteractives/Laser/BPI_LightBeams.LightBeam Bounce` _lasthitactor self false (struct))))

(event `self.ReceiveTick`
  (params (DeltaSeconds :type "Float (single-precision)"))
  (`self.Generate LightBeam` (`self.Ray Ignore`)))

(fn `Generate LightBeam`
  (params (RayIgnore :type "Array of Actor Object Reference"))
  (locals (L_Range :type "Float (double-precision)" :default 3000.0) (L_Hit :type "HitResult Structure") (L_HitActor :type "Actor Object Reference"))
  (bind _returnvalue (`self.GetActorUpVector`))
  (bind _lasthitactor (`self.LastHitActor`))
  (bind _l_range (`local.L_Range`))
  (bind _l_hitactor (`local.L_HitActor`))
  (bind _returnvalue_2 (+ (`self.K2_GetActorLocation`) (* _returnvalue 2.0)))
  (bind _outhit (`KismetSystemLibrary.BoxTraceSingle` _returnvalue_2 (+ _returnvalue_2 (* _returnvalue (`local.L_Range`))) (0.5 0.5 0.5) (struct) "TraceTypeQuery1" false RayIgnore))
  (bind _output_get (set `local.L_Hit` _outhit))
  (bind (_bblockinghit _binitialoverlap _time _distance _location _impactpoint _normal _impactnormal _physmat _hitactor) (`GameplayStatics.BreakHitResult` _output_get))
  (set `local.L_HitActor` _hitactor)
  (bind _returnvalue_3 (`KismetMathLibrary.SelectFloat` (/ (+ _distance 1.0) 100.0) (/ _l_range 100.0) _bblockinghit))
  (`SceneComponent.SetWorldScale3D` (`self.LightBeamMesh`) (`KismetMathLibrary.MakeVector` 0.1 0.1 _returnvalue_3))
  (for _array_element (`self.LightsList`)
    (`RectLightComponent.SetSourceHeight` _array_element (* _returnvalue_3 100.0))
    (`LocalLightComponent.SetAttenuationRadius` _array_element _l_range))
  (bind _output_get_2 (set `self.Sound Attenuation Settings` (make `SoundAttenuationSettings` :`DistanceAlgorithm` "Inverse" :`AttenuationShape` "Box" :`AttenuationShapeExtents` (`KismetMathLibrary.MakeVector` 30.0 60.0 (* _returnvalue_3 50.0)))))
  (`AudioComponent.AdjustAttenuation` (`self.Audio`) _output_get_2)
  (`|ExecutionSequence`
    (:`then_0`
      (if (!= (`self.LastHitActor`) (`local.L_HitActor`))
        (if (`KismetSystemLibrary.DoesImplementInterface` _lasthitactor "/Game/WallFContent/BluePrint/EnvironmentInteractives/Laser/BPI_LightBeams.BPI_LightBeams_C")
          (message `/Game/WallFContent/BluePrint/EnvironmentInteractives/Laser/BPI_LightBeams.LightBeam Bounce` _lasthitactor self false (`local.L_Hit`))
          (set `self.wasChanged` false))
        (elif (`KismetSystemLibrary.DoesImplementInterface` _l_hitactor "/Game/WallFContent/BluePrint/EnvironmentInteractives/Laser/BPI_LightBeams.BPI_LightBeams_C")
          (if (`self.wasChanged`)
            (bind _return (message `/Game/WallFContent/BluePrint/EnvironmentInteractives/Laser/BPI_LightBeams.Bounce Update` _l_hitactor (`self.NextBeam`) (`local.L_Hit`)))
            (set `self.NextBeam` _return)
            (else
              (bind _new_lightbeam (message `/Game/WallFContent/BluePrint/EnvironmentInteractives/Laser/BPI_LightBeams.LightBeam Bounce` _l_hitactor self true (`local.L_Hit`)))
              (set `self.NextBeam` _new_lightbeam)
              (set `self.wasChanged` true))))))
    (:`then_1`
      (bind _l_hitactor_2 (`local.L_HitActor`)
        (:`then`
          (set `self.LastHitActor` _l_hitactor_2))
        (:`else`)))))

(fn `Set Color`
  (bind _color (`self.Color`))
  (bind _returnvalue (`PrimitiveComponent.CreateDynamicMaterialInstance` (`self.LightBeamMesh`) 0 "/Game/WallFContent/BluePrint/EnvironmentInteractives/Laser/M_LightBeam.M_LightBeam" "None"))
  (`MaterialInstanceDynamic.SetVectorParameterValue` _returnvalue "Color" (`self.Color`))
  (for _array_element (`self.LightsList`)
    (`LightComponent.SetLightColor` _array_element _color true)
    (`LightComponent.SetLightColor` (`self.ImpactLight`) _color true)))

(fn `Update ID`
  (params (`Append ID` :type String))
  (returns (`Return ID` :type String))
  (return (`KismetStringLibrary.Concat_StrStr` (`self.Beam_ID`) `Append ID`)))

(fn `UserConstructionScript`)