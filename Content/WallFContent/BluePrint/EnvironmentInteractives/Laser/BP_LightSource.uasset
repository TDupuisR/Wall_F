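; Laser light source for environment interactives that emits a colored BP_LightBeam from its Arrow position and can be switched on and off.
; Each beam is attached to the source, tagged with a beam ID, set to ignore itself and tracked in BeamList for teardown.
; Call spawns or destroys beams, inverting the signal if the source started active.
; CheckID tests whether an asker's ID contains this source's ID.
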(event `self.ReceiveBeginPlay`
  (bind _isactive (`self.IsActive`))
  (set `self.Invert` _isactive)
  (if _isactive
    (set `self.LightID` (`KismetSystemLibrary.GetDisplayName` self))
    (bind _returnvalue (`|SpawnActorFromClass` "/Game/WallFContent/BluePrint/EnvironmentInteractives/Laser/BP_LightBeam.BP_LightBeam_C" (`KismetMathLibrary.MakeTransform` (`SceneComponent.K2_GetComponentLocation` (`self.Arrow`)) (`SceneComponent.K2_GetComponentRotation` (`self.Source`)) (0.5 0.5 0.5)) "Undefined" "MultiplyWithRoot" null (`self.Color`) (`self.LightID`) self null :!label _label))
    (`self.K2_AttachToActor` _returnvalue self "None" "KeepWorld" "KeepWorld" "KeepWorld" true)
    (`KismetArrayLibrary.Array_Add` (`/Game/WallFContent/BluePrint/EnvironmentInteractives/Laser/BP_LightBeam.Ray Ignore` _returnvalue) _returnvalue)
    (`KismetArrayLibrary.Array_Add` (`self.BeamList`) _returnvalue)))

(event `/Game/WallFContent/BluePrint/EnvironmentInteractives/PressurePlate/I_Link.Call`
  (params (ActorID :type String) (IsActive :type Boolean))
  (bind _beamlist (`self.BeamList`))
  (if (`self.Invert`)
    (if IsActive
      _
      (else
        (goto _label)))
    (elif IsActive
      (goto _label)
      (else
        _)))
  (for _array_element _beamlist
    (`/Engine/EditorBlueprintResources/StandardMacros.IsValid` _array_element
      (:`Is Valid`
        (`/Game/WallFContent/BluePrint/EnvironmentInteractives/Laser/BP_LightBeam.DestroyFunction` _array_element))))
  (`KismetArrayLibrary.Array_Clear` _beamlist))

(fn `CheckID`
  (params (AskerID :type String))
  (returns (IsSame :type Boolean))
  (bind _id (`self.ID`))
  (if (`KismetStringLibrary.IsEmpty` _id)
    (return false)
    (else
      (return (`KismetStringLibrary.Contains` AskerID _id)))))

(fn `UserConstructionScript`)