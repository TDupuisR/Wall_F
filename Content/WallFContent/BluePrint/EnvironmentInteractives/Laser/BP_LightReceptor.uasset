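; Laser receptor interactive that switches on or off when a light beam reports a hit and signals the actors linked to it.
; On BeginPlay it gathers every I_Link actor that accepts its ID as a receiver.
; Each beam bounce event stores the hit response as Active, forwards it to those receivers, then creates a dynamic material on the panel, glowing in the beam's color when active and unlit otherwise.
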(event `self.ReceiveBeginPlay`
  (set `self.Active` false)
  (`self.FindID` (`self.ID`)))

(event `/Game/WallFContent/BluePrint/EnvironmentInteractives/PressurePlate/I_Link.FindID`
  (params (ID :type String))
  (bind _outactors (`GameplayStatics.GetAllActorsWithInterface` "/Game/WallFContent/BluePrint/EnvironmentInteractives/PressurePlate/I_Link.I_Link_C"))
  (for _array_element _outactors
    (bind _issame (message `/Game/WallFContent/BluePrint/EnvironmentInteractives/PressurePlate/I_Link.CheckID` _array_element ID))
    (if _issame
      (`KismetArrayLibrary.Array_Add` (`self.Receiver`) _array_element))))

(event `/Game/WallFContent/BluePrint/EnvironmentInteractives/PressurePlate/I_Link.Call`
  (params (ActorID :type String) (IsActive :type Boolean)))

(fn `ActivateSensor`
  (params (Color :type "LinearColor Structure"))
  (bind _active (`self.Active`))
  (bind _returnvalue (`PrimitiveComponent.CreateDynamicMaterialInstance` (`self.Panel`) 3 "/Game/WallFContent/ART/02_Materials/Spotlight/Ampoule_Spotlight.Ampoule_Spotlight" "None"))
  (`MaterialInstanceDynamic.SetVectorParameterValue` _returnvalue "Param" (`KismetMathLibrary.SelectColor` Color (struct :`R` 0.799103 :`G` 0.708376 :`B` 0.114435 :`A` 1.0) _active))
  (`MaterialInstanceDynamic.SetScalarParameterValue` _returnvalue "Intensity" (`KismetMathLibrary.SelectFloat` 20.0 0.0 _active)))

(fn `Bounce Update`
  (params (LightBeam :type "/Game/WallFContent/BluePrint/EnvironmentInteractives/Laser/BP_LightBeam Object Reference") (Hit :type "HitResult Structure"))
  (returns (Return :type "/Game/WallFContent/BluePrint/EnvironmentInteractives/Laser/BP_LightBeam Object Reference"))
  (return null))

(fn `CheckID`
  (params (AskerID :type String))
  (returns (IsSame :type Boolean))
  (return false))

(fn `LightBeam Bounce`
  (params (LightBeamHit :type "/Game/WallFContent/BluePrint/EnvironmentInteractives/Laser/BP_LightBeam Object Reference") (HitResponse :type Boolean) (HitInfo :type "HitResult Structure"))
  (returns (New_LightBeam :type "/Game/WallFContent/BluePrint/EnvironmentInteractives/Laser/BP_LightBeam Object Reference"))
  (bind _output_get (set `self.Active` HitResponse))
  (for _array_element (`self.Receiver`)
    (message `/Game/WallFContent/BluePrint/EnvironmentInteractives/PressurePlate/I_Link.Call` _array_element (`self.ID`) _output_get))
  (`self.ActivateSensor` (`/Game/WallFContent/BluePrint/EnvironmentInteractives/Laser/BP_LightBeam.Color` LightBeamHit))
  (return null))

(fn `UserConstructionScript`)