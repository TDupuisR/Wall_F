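; BP_Magnet is an interactive environment magnet that registers itself with metal objects entering its trigger zone.
; Overlapping actors with a BPC_MetalBehaviour component get the magnet added to their MagnetInfos list, and removed when they leave.
; It stores the Magnet-to-TriggerZone distance as MaxDistance at BeginPlay, and ChangePolarity_Event flips its Repulse flag.
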(event `self.ReceiveBeginPlay`
  (set `self.MaxDistance` (`KismetMathLibrary.Vector_Distance` (`SceneComponent.RelativeLocation` (`self.Magnet`)) (`SceneComponent.RelativeLocation` (`self.TriggerZone`)))))

(event `self.TriggerZone.OnComponentBeginOverlap`
  (params (OverlappedComponent :type "PrimitiveComponent Object Reference") (OtherActor :type "Actor Object Reference") (OtherComp :type "PrimitiveComponent Object Reference") (OtherBodyIndex :type Integer) (bFromSweep :type Boolean) (SweepResult :type "HitResult Structure (by ref)"))
  (bind _returnvalue (`self.GetComponentByClass` OtherActor "/Game/WallFContent/BluePrint/Cube/BPC_MetalBehaviour.BPC_MetalBehaviour_C"))
  (`/Engine/EditorBlueprintResources/StandardMacros.IsValid` _returnvalue
    (:`Is Valid`
      (`KismetArrayLibrary.Array_AddUnique` (`/Game/WallFContent/BluePrint/Cube/BPC_MetalBehaviour.MagnetInfos` _returnvalue) self))))

(event `self.TriggerZone.OnComponentEndOverlap`
  (params (OverlappedComponent :type "PrimitiveComponent Object Reference") (OtherActor :type "Actor Object Reference") (OtherComp :type "PrimitiveComponent Object Reference") (OtherBodyIndex :type Integer))
  (bind _returnvalue (`self.GetComponentByClass` OtherActor "/Game/WallFContent/BluePrint/Cube/BPC_MetalBehaviour.BPC_MetalBehaviour_C"))
  (`/Engine/EditorBlueprintResources/StandardMacros.IsValid` _returnvalue
    (:`Is Valid`
      (`KismetArrayLibrary.Array_RemoveItem` (`/Game/WallFContent/BluePrint/Cube/BPC_MetalBehaviour.MagnetInfos` _returnvalue) self))))

(event `ChangePolarity_Event`
  (set `self.Repulse` (not (`self.Repulse`))))

(fn `UserConstructionScript`)