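; BP_ManagerIncinerator is a level manager that counts incinerator completion events and activates linked actors once more than two have fired.
; On BeginPlay it binds to every BP_Incinerator's finish event and caches I_Link actors that match its ID as receivers.
; Past the threshold, it sends them an active message, with debug prints indicating a third-level unlock.
; Its own CheckID always returns false.
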(event `self.ReceiveBeginPlay`
  (bind _outactors (`GameplayStatics.GetAllActorsOfClass` "/Game/WallFContent/BluePrint/EnvironmentInteractives/BP_Incinerator.BP_Incinerator_C"))
  (bind _output_get (set `self.Incinerators` _outactors))
  (for _array_element _output_get
    (add `/Game/WallFContent/BluePrint/EnvironmentInteractives/BP_Incinerator.ED_Finish` _array_element (delegate `CustomEvent`)))
  (`/Game/WallFContent/BluePrint/EnvironmentInteractives/PressurePlate/I_Link.FindID` (`self.ID`)))

(event `CustomEvent`
  (bind _output_get (set `self.LevelFinished` (+ (`self.LevelFinished`) 1)))
  (`KismetSystemLibrary.PrintString` (`KismetStringLibrary.Concat_StrStr` "N Levels Finished :" (`KismetStringLibrary.Conv_IntToString` _output_get)))
  (if (> (`self.LevelFinished`) 2)
    (`KismetSystemLibrary.PrintString` "Unlock 3e niveau")
    (for _array_element (`self.Receivers`)
      (message `/Game/WallFContent/BluePrint/EnvironmentInteractives/PressurePlate/I_Link.Call` _array_element (`self.ID`) true))))

(event `/Game/WallFContent/BluePrint/EnvironmentInteractives/PressurePlate/I_Link.FindID`
  (params (ID :type String))
  (bind _outactors (`GameplayStatics.GetAllActorsWithInterface` "/Game/WallFContent/BluePrint/EnvironmentInteractives/PressurePlate/I_Link.I_Link_C"))
  (for _array_element _outactors
    (bind _issame (message `/Game/WallFContent/BluePrint/EnvironmentInteractives/PressurePlate/I_Link.CheckID` _array_element ID))
    (if _issame
      (`KismetArrayLibrary.Array_Add` (`self.Receivers`) _array_element))))

(fn `CheckID`
  (params (AskerID :type String))
  (returns (IsSame :type Boolean))
  (return false))

(fn `UserConstructionScript`)