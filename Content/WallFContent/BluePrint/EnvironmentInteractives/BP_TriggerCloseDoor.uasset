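; One-shot trigger volume, named for closing doors, that activates linked actors when a BP_Character enters its box collider.
; On BeginPlay it gathers every I_Link actor that confirms the trigger's ID into a Receivers list.
; The first character overlap sends each receiver an active call with that ID and sets Used to block repeats.
; Its own CheckID always returns false.
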(event `self.ReceiveBeginPlay`
  (`/Game/WallFContent/BluePrint/EnvironmentInteractives/PressurePlate/I_Link.FindID` (`self.ID`)))

(event `/Game/WallFContent/BluePrint/EnvironmentInteractives/PressurePlate/I_Link.FindID`
  (params (ID :type String))
  (bind _outactors (`GameplayStatics.GetAllActorsWithInterface` "/Game/WallFContent/BluePrint/EnvironmentInteractives/PressurePlate/I_Link.I_Link_C"))
  (for _array_element _outactors
    (bind _issame (message `/Game/WallFContent/BluePrint/EnvironmentInteractives/PressurePlate/I_Link.CheckID` _array_element ID))
    (if _issame
      (`KismetArrayLibrary.Array_Add` (`self.Receivers`) _array_element))))

(event `self.BoxCollider.OnComponentBeginOverlap`
  (params (OverlappedComponent :type "PrimitiveComponent Object Reference") (OtherActor :type "Actor Object Reference") (OtherComp :type "PrimitiveComponent Object Reference") (OtherBodyIndex :type Integer) (bFromSweep :type Boolean) (SweepResult :type "HitResult Structure (by ref)"))
  (if (not (`self.Used`))
    (cast `/Game/WallFContent/BluePrint/BP_Character` OtherActor)
    (for _array_element (`self.Receivers`)
      (message `/Game/WallFContent/BluePrint/EnvironmentInteractives/PressurePlate/I_Link.Call` _array_element (`self.ID`) true)
      (set `self.Used` true))))

(fn `CheckID`
  (params (AskerID :type String))
  (returns (IsSame :type Boolean))
  (return false))

(fn `UserConstructionScript`)