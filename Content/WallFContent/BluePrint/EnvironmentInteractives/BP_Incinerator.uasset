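; BP_Incinerator is a puzzle goal that destroys cubes dropped into its trigger box once enough are inside.
; It tracks I_Cube overlaps and, while unlocked, ends the speedrun split, plays validation audio, destroys the cubes and activates I_Link receivers matched by ID at BeginPlay.
; It then locks, optionally calls a player teleport dispatcher and fires a finish dispatcher.
; CE_CallEditorable triggers only that final lock, teleport and finish stage.
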(event `self.ReceiveBeginPlay`
  (`/Game/WallFContent/BluePrint/EnvironmentInteractives/PressurePlate/I_Link.FindID` (`self.ID`))
  (`AudioComponent.Play` (`self.Audio`) 0.0)
  (bind _returnvalue (`GameplayStatics.GetActorOfClass` "/Game/WallFContent/BluePrint/Speedrun/BP_SpeedrunManager.BP_SpeedrunManager_C"))
  (set `self.SpeedrunManager` _returnvalue))

(event `self.Box.OnComponentBeginOverlap`
  (params (OverlappedComponent :type "PrimitiveComponent Object Reference") (OtherActor :type "Actor Object Reference") (OtherComp :type "PrimitiveComponent Object Reference") (OtherBodyIndex :type Integer) (bFromSweep :type Boolean) (SweepResult :type "HitResult Structure (by ref)"))
  (bind _nbloc (`self.NBloc`))
  (if (`KismetSystemLibrary.DoesImplementInterface` OtherActor "/Game/WallFContent/BluePrint/Cube/I_Cube.I_Cube_C")
    (bind _asi_cube (cast `/Game/WallFContent/BluePrint/Cube/I_Cube` OtherActor))
    (if (not (`KismetArrayLibrary.Array_Contains` _nbloc _asi_cube))
      (`KismetArrayLibrary.Array_Add` _nbloc _asi_cube)
      (if (and (>= (`KismetArrayLibrary.Array_Length` _nbloc) (`self.NbBlocNeeded`)) (`self.IsUnlocked`))
        (`/Game/WallFContent/BluePrint/Speedrun/BP_SpeedrunManager.EndCurrentSplit` (`self.SpeedrunManager`))
        (`AudioParameterControllerInterface.SetTriggerParameter` (`self.Audio`) "Validate")
        (for _array_element (`self.NBloc`)
          (bind _selfobj (`/Game/WallFContent/BluePrint/Cube/I_Cube.I_GetSelf` _array_element))
          (`self.K2_DestroyActor` _selfobj))
        (for _array_element_2 (`self.Receivers`)
          (message `/Game/WallFContent/BluePrint/EnvironmentInteractives/PressurePlate/I_Link.Call` _array_element_2 (`self.ID`) true))
        (set `self.IsUnlocked` false :!label _label)
        (if (`self.tp`)
          (`self.ED_Teleport` (`SceneComponent.K2_GetComponentLocation` (`self.TPJoueur`)) (`self.Delay Incinerator`) true))
        (`self.ED_Finish`)))))

(event `CE_CallEditorable`
  (goto _label))

(event `self.Box.OnComponentEndOverlap`
  (params (OverlappedComponent :type "PrimitiveComponent Object Reference") (OtherActor :type "Actor Object Reference") (OtherComp :type "PrimitiveComponent Object Reference") (OtherBodyIndex :type Integer))
  (bind _nbloc (`self.NBloc`))
  (if (`KismetSystemLibrary.DoesImplementInterface` OtherActor "/Game/WallFContent/BluePrint/Cube/I_Cube.I_Cube_C")
    (bind _asi_cube (cast `/Game/WallFContent/BluePrint/Cube/I_Cube` OtherActor))
    (if (`KismetArrayLibrary.Array_Contains` _nbloc _asi_cube)
      (`KismetArrayLibrary.Array_RemoveItem` _nbloc _asi_cube))))

(event `/Game/WallFContent/BluePrint/EnvironmentInteractives/PressurePlate/I_Link.FindID`
  (params (ID :type String))
  (bind _outactors (`GameplayStatics.GetAllActorsWithInterface` "/Game/WallFContent/BluePrint/EnvironmentInteractives/PressurePlate/I_Link.I_Link_C"))
  (for _array_element _outactors
    (bind _issame (message `/Game/WallFContent/BluePrint/EnvironmentInteractives/PressurePlate/I_Link.CheckID` _array_element ID))
    (if _issame
      (`KismetArrayLibrary.Array_Add` (`self.Receivers`) _array_element))))

(event `/Game/WallFContent/BluePrint/EnvironmentInteractives/PressurePlate/I_Link.Call`
  (params (ActorID :type String) (IsActive :type Boolean)))

(fn `CheckID`
  (params (AskerID :type String))
  (returns (IsSame :type Boolean))
  (if (`KismetStringLibrary.IsEmpty` (`self.ID`))
    (return false)))

(fn `UserConstructionScript`)