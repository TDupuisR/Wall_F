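; HUD_Game is the in-game HUD that creates the game's UI widgets when play begins.
; It adds end screen, speedrun timer, pause menu, options, controls and cheats widgets to the viewport up front, storing each in a variable and starting the menus hidden.
; The timer shows only when the game instance flags a speedrun.
; Finally it finds BP_ManagerCheats and calls its CESETUP, after all widgets exist.
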(event `self.ReceiveBeginPlay`
  (bind _returnvalue (`|CreateWidget` "/Game/WallFContent/Widgets/W_EndScreen.W_EndScreen_C"))
  (bind _output_get (set `self.EndScreen` _returnvalue))
  (`UserWidget.AddToViewport` _output_get 0)
  (`Widget.SetVisibility` _returnvalue "Hidden")
  (bind _returnvalue_2 (`|CreateWidget` "/Game/WallFContent/Widgets/W_SpeedrunTimer.W_SpeedrunTimer_C"))
  (bind _output_get_2 (set `self.Timer` _returnvalue_2))
  (`UserWidget.AddToViewport` _output_get_2 0)
  (bind _asgi_game_instance (cast `/Game/WallFContent/BluePrint/GI_GameInstance` (`GameplayStatics.GetGameInstance`)))
  (bind _output_get_3 (set `self.GameInstance` _asgi_game_instance))
  (if (`/Game/WallFContent/BluePrint/GI_GameInstance.InSpeedrun` _output_get_3)
    (`Widget.SetVisibility` _output_get_2 "SelfHitTestInvisible")
    (else
      (`Widget.SetVisibility` _output_get_2 "Hidden")))
  (bind _returnvalue_3 (`|CreateWidget` "/Game/WallFContent/Widgets/W_PauseMenu.W_PauseMenu_C"))
  (bind _output_get_4 (set `self.PauseMenu` _returnvalue_3))
  (`UserWidget.AddToViewport` _output_get_4 0)
  (`Widget.SetVisibility` _output_get_4 "Hidden")
  (bind _returnvalue_4 (`|CreateWidget` "/Game/WallFContent/Widgets/W_Options.W_Options_C"))
  (bind _output_get_5 (set `self.Options` _returnvalue_4))
  (`UserWidget.AddToViewport` _output_get_5 0)
  (`Widget.SetVisibility` _output_get_5 "Hidden")
  (bind _returnvalue_5 (`|CreateWidget` "/Game/WallFContent/Widgets/W_Controles.W_Controles_C"))
  (bind _output_get_6 (set `self.Controles` _returnvalue_5))
  (`UserWidget.AddToViewport` _output_get_6 0)
  (`Widget.SetVisibility` _output_get_6 "Hidden")
  (bind _returnvalue_6 (`|CreateWidget` "/Game/WallFContent/Widgets/W_Cheats.W_Cheats_C"))
  (bind _output_get_7 (set `self.Cheats` _returnvalue_6))
  (`UserWidget.AddToViewport` _output_get_7 0)
  (`Widget.SetVisibility` _output_get_7 "Hidden")
  (bind _returnvalue_7 (`GameplayStatics.GetActorOfClass` "/Game/WallFContent/BluePrint/BP_ManagerCheats.BP_ManagerCheats_C"))
  (`/Game/WallFContent/BluePrint/BP_ManagerCheats.CE_SETUP` _returnvalue_7))

(fn `UserConstructionScript`)