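; BP_ManagerCheckpointsPresentation is a manager that moves the player between presentation checkpoints, each tagged with a Level value.
; On BeginPlay it caches the player's BP_Character and gathers every BP_CheckpointPresentation in the world.
; GoToCheckpoint calls PlayerTP on checkpoints matching the requested Level and records it as LastLevel.
; GoToNextCheckpoint uses LastLevel to cycle through Ferdi, Paul and Daphne in a loop.
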(event `self.ReceiveBeginPlay`
  (bind _asbp_character (cast `/Game/WallFContent/BluePrint/BP_Character` (`GameplayStatics.GetPlayerCharacter` 0)))
  (set `self.Character` _asbp_character)
  (bind _outactors (`GameplayStatics.GetAllActorsOfClass` "/Game/WallFContent/BluePrint/Presentation/BP_CheckpointPresentation.BP_CheckpointPresentation_C"))
  (set `self.Checkpoints` _outactors))

(event `GoToNextCheckpoint`
  (switch `/Game/WallFContent/BluePrint/Speedrun/E_SplitName` (`self.LastLevel`)
    (:`NewEnumerator2`
      (`self.GoToCheckpoint` "NewEnumerator3"))
    (:`NewEnumerator3`
      (`self.GoToCheckpoint` "NewEnumerator4"))
    (:`NewEnumerator4`
      (`self.GoToCheckpoint` "NewEnumerator2"))))

(event `GoToCheckpoint`
  (params (Level :type "/Game/WallFContent/BluePrint/Speedrun/E_SplitName Enum" :default "NewEnumerator0"))
  (for _array_element (`self.Checkpoints`)
    (if (`|EnumEquality` (`/Game/WallFContent/BluePrint/Presentation/BP_CheckpointPresentation.Level` _array_element) Level)
      (`/Game/WallFContent/BluePrint/Presentation/BP_CheckpointPresentation.PlayerTP` _array_element)
      (set `self.LastLevel` Level))))

(fn `UserConstructionScript`)