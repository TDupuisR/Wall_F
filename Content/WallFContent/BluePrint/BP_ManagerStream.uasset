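; BP_ManagerStream watches level streaming and signals when streamed levels finish loading.
; On BeginPlay, outside IntegrationScene, it gathers every LevelStreamingVolume and binds a custom event to the OnLevelLoaded of each streaming level the volumes name.
; That event fires the CEONLOADED dispatcher on each load, relaying all of them through one point.
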(event `self.ReceiveBeginPlay`
  (bind _returnvalue (`GameplayStatics.GetCurrentLevelName` true))
  (if (not (`KismetStringLibrary.EqualEqual_StrStr` _returnvalue "IntegrationScene"))
    (bind _outactors (`GameplayStatics.GetAllActorsOfClass` "/Script/Engine.LevelStreamingVolume"))
    (bind _output_get (set `self.streams` _outactors))
    (for _array_element _output_get
      (for _array_element_2 (`LevelStreamingVolume.StreamingLevelNames` _array_element)
        (add `LevelStreaming.OnLevelLoaded` (`GameplayStatics.GetStreamingLevel` _array_element_2) (delegate `CustomEvent`))))))

(event `CustomEvent`
  (`self.CE_ONLOADED`))

(fn `UserConstructionScript`)