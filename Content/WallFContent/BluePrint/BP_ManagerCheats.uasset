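; Cheat manager that spawns test cubes in front of or around the player on requests from the game HUD's Cheats element.
; CE_SETUP, not called within this Blueprint, binds to the Cheats spawn and level events and caches the character's SpawnCheats component.
; Spawn switches on the name to create a BP_Cube at that component, adding a plastic, metal or rubber behaviour component plus buoyancy.
; The level cheat is wired but its function is empty.
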(event `self.ReceiveBeginPlay`)

(event `CE_SETUP`
  (bind _ashud_game (cast `/Game/WallFContent/BluePrint/HUD_Game` (`PlayerController.GetHUD` (`GameplayStatics.GetPlayerController` 0))))
  (bind _cheats (`/Game/WallFContent/BluePrint/HUD_Game.Cheats` _ashud_game))
  (add `/Game/WallFContent/Widgets/W_Cheats.Spawn` _cheats (delegate `CE_Spawn`))
  (add `/Game/WallFContent/Widgets/W_Cheats.CheatLVL` _cheats (delegate `CE_SetLVL`))
  (bind _asbp_character (cast `/Game/WallFContent/BluePrint/BP_Character` (`GameplayStatics.GetPlayerCharacter` 0)))
  (bind _output_get (set `self.As BP Character` _asbp_character))
  (set `self.Spawn Cheats` (`/Game/WallFContent/BluePrint/BP_Character.SpawnCheats` _output_get)))

(event `CE_Spawn`
  (params (Name :type String))
  (`self.Spawn` Name))

(event `CE_SetLVL`
  (params (LVL :type Integer))
  (`self.LVL` LVL))

(fn `LVL`
  (params (LVL :type Integer)))

(fn `Spawn`
  (params (Name :type String))
  (bind _returnvalue (`SceneComponent.K2_GetComponentLocation` (`self.Spawn Cheats`)))
  (switch `string` Name
    (:`CubePlastic`
      (bind _returnvalue_2 (`|SpawnActorFromClass` "/Game/WallFContent/BluePrint/Cube/BP_Cube.BP_Cube_C" (`KismetMathLibrary.MakeTransform` _returnvalue) "AdjustIfPossibleButAlwaysSpawn" "MultiplyWithRoot" null false null))
      (`AddComponent|NODE_AddBPC_PlasticBehaviour-0` :`self` _returnvalue_2)
      (`AddComponent|NODE_AddBPC_Buoyancy-1` :`self` _returnvalue_2))
    (:`CubeMetal`
      (bind _returnvalue_3 (`|SpawnActorFromClass` "/Game/WallFContent/BluePrint/Cube/BP_Cube.BP_Cube_C" (`KismetMathLibrary.MakeTransform` _returnvalue) "AdjustIfPossibleButAlwaysSpawn" "MultiplyWithRoot" null false null))
      (`AddComponent|NODE_AddBPC_MetalBehaviour-0` :`self` _returnvalue_3)
      (`AddComponent|NODE_AddBPC_Buoyancy-2` :`self` _returnvalue_3))
    (:`CubeRubber`
      (bind _returnvalue_4 (`|SpawnActorFromClass` "/Game/WallFContent/BluePrint/Cube/BP_Cube.BP_Cube_C" (`KismetMathLibrary.MakeTransform` _returnvalue) "AdjustIfPossibleButAlwaysSpawn" "MultiplyWithRoot" null false null))
      (`AddComponent|NODE_AddBPC_RubberBehaviour-0` :`self` _returnvalue_4)
      (`AddComponent|NODE_AddBPC_Buoyancy-3` :`self` _returnvalue_4))))

(fn `UserConstructionScript`)