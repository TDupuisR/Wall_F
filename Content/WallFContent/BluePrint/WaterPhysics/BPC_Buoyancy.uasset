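; Actor component that makes a BP_Cube float and drift in BP_WaterBody volumes.
; Cube overlap events track water bodies, summing their flow, raising the surface height to the highest top, setting InWater and playing a splash on entry.
; Each tick in water, "Buoyancy"-tagged static meshes act as sample points for depth-scaled Archimedes lift, linear drag and angular drag.
; Flow pushes the cube even with buoyancy disabled.
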(event `self.ReceiveBeginPlay`
  (bind _returnvalue (`self.GetOwner`))
  ;[1 0.1269 0.1448] Begin Initialization
  (set `self.GravityZ` -980.0)
  (set `self.WaterFlowForce` (0.0 0.0 0.0))
  (bind _output_get (set `self.BuoList` (`Actor.GetComponentsByTag` _returnvalue "/Script/Engine.StaticMeshComponent" "Buoyancy")))
  (bind _output_get_2 (set `self.BuoAmount` (`KismetArrayLibrary.Array_Length` _output_get)))
  (if (<= _output_get_2 0)
    (set `self.Buoyancy` false))
  (bind _asbp_cube (cast `/Game/WallFContent/BluePrint/Cube/BP_Cube` _returnvalue)
    (:`then`
      (add `/Game/WallFContent/BluePrint/Cube/BP_Cube.OnCubeOverlapBegin` _asbp_cube (delegate `Cube Begin Overlap`))
      (add `/Game/WallFContent/BluePrint/Cube/BP_Cube.OnCubeOverlapEnd` _asbp_cube (delegate `Cube End Overlap`))
      (`KismetArrayLibrary.Array_Clear` (`self.WaterBodyList`))
      (set `self.WaterZTop` -100000000000000.0)
      (set `self.Cube` (`/Game/WallFContent/BluePrint/Cube/BP_Cube.Cube` _asbp_cube))
      (set `self.As BP Cube` _asbp_cube))
    (:`CastFailed`
      (`KismetSystemLibrary.LogString` (`KismetStringLibrary.Concat_StrStr` (`KismetSystemLibrary.GetDisplayName` _returnvalue) " -> BPC_Buoyancy : Cast Failed (Owner -> BP_Cube)")))))

(event `Cube Begin Overlap`
  (params (`Other Actor` :type "Actor Object Reference"))
  (bind _asbp_water_body (cast `/Game/WallFContent/BluePrint/WaterPhysics/BP_WaterBody` `Other Actor`))
  (`KismetArrayLibrary.Array_Add` (`self.WaterBodyList`) _asbp_water_body)
  (`AudioParameterControllerInterface.SetTriggerParameter` (`/Game/WallFContent/BluePrint/Cube/BP_Cube.Audio` (`self.As BP Cube`)) "Plouf")
  (set `self.WaterFlowForce` (0.0 0.0 0.0) :!label _label)
  (for _array_element (`self.WaterBodyList`)
    (set `self.WaterFlowForce` (+ (`self.WaterFlowForce`) (`/Game/WallFContent/BluePrint/WaterPhysics/BP_WaterBody.WaterFlow` _array_element)))
    (bind (_returnvalue_x _returnvalue_y _returnvalue_z) (`KismetMathLibrary.BreakVector` (`SceneComponent.K2_GetComponentLocation` (`Actor.RootComponent` _array_element))))
    (bind _returnvalue (+ _returnvalue_z (`/Game/WallFContent/BluePrint/WaterPhysics/BP_WaterBody.BoxZOffset` _array_element)))
    (if (> _returnvalue (`self.WaterZTop`))
      (set `self.WaterZTop` _returnvalue)))
  (bind _output_get (set `self.InWater` true))
  (set `/Game/WallFContent/BluePrint/Cube/BP_Cube.inWater` _output_get (`self.As BP Cube`)))

(event `Cube End Overlap`
  (params (`Other Actor` :type "Actor Object Reference"))
  (bind _waterbodylist (`self.WaterBodyList`))
  (bind _asbp_water_body (cast `/Game/WallFContent/BluePrint/WaterPhysics/BP_WaterBody` `Other Actor`))
  (`KismetArrayLibrary.Array_RemoveItem` _waterbodylist _asbp_water_body)
  (if (> (`KismetArrayLibrary.Array_Length` _waterbodylist) 0)
    (goto _label)
    (else
      (bind _output_get (set `self.InWater` false))
      (set `/Game/WallFContent/BluePrint/Cube/BP_Cube.inWater` _output_get (`self.As BP Cube`))
      (set `self.WaterZTop` -100000000000000.0))))

(event `self.ReceiveTick`
  (params (DeltaSeconds :type "Float (single-precision)"))
  (bind _returnvalue (`GameplayStatics.GetWorldDeltaSeconds`))
  (bind _cube (`self.Cube`))
  (if (and (`self.InWater`) (`self.Buoyancy`))
    ;[1 0.8122 0.4064] Init Variables & Loop
    (for _array_element (`self.BuoList`)
      (bind _returnvalue_2 (`SceneComponent.K2_GetComponentLocation` _array_element))
      (bind (_returnvalue_x _returnvalue_y _returnvalue_z) (`KismetMathLibrary.BreakVector` (+ _returnvalue_2 (0.0 0.0 0.0))))
      (bind _returnvalue_3 (* (`self.BuoAppliedForce`) (`KismetMathLibrary.FClamp` (`KismetMathLibrary.SafeDivide` (- (`self.WaterZTop`) _returnvalue_z) (`self.BuoDepth`)) 0.0 1000.0) 0.1))
      ;[0.3017 0.4763 1] Archimedes' principle
      (`PrimitiveComponent.AddForceAtLocation` _cube (`KismetMathLibrary.MakeVector` 0.0 0.0 (/ (* _returnvalue_3 (`KismetMathLibrary.Abs` (`self.GravityZ`))) (`self.BuoAmount`))) _returnvalue_2 "None")
      (bind (_returnvalue_x_2 _returnvalue_y_2 _returnvalue_z_2) (`KismetMathLibrary.BreakVector` (* _returnvalue _returnvalue_3 (`self.BuoDragForce`) (`KismetMathLibrary.NegateVector` (`SceneComponent.GetComponentVelocity` _cube)))))
      ;[0.3992 0.3637 1] Fluid Drag Force
      (`PrimitiveComponent.AddForceAtLocation` _cube (`KismetMathLibrary.MakeVector` (/ _returnvalue_x_2 (`self.BuoAmount`)) (/ _returnvalue_y_2 (`self.BuoAmount`)) (/ _returnvalue_z_2 (`self.BuoAmount`))) _returnvalue_2 "None")
      (bind (_returnvalue_x_3 _returnvalue_y_3 _returnvalue_z_3) (`KismetMathLibrary.BreakVector` (* _returnvalue _returnvalue_3 (`self.BuoAngularDragForce`) (`KismetMathLibrary.NegateVector` (`PrimitiveComponent.GetPhysicsAngularVelocityInRadians` _cube "None")))))
      ;[0.4325 1 0.8735] Angular Drag Force
      (`PrimitiveComponent.AddTorqueInRadians` _cube (`KismetMathLibrary.MakeVector` (/ _returnvalue_x_3 (`self.BuoAmount`)) (/ _returnvalue_y_3 (`self.BuoAmount`)) (/ _returnvalue_z_3 (`self.BuoAmount`))) "None" true))
    (`PrimitiveComponent.AddForce` _cube (`self.WaterFlowForce`) "None" true :!label _label_2)
    (elif (`self.InWater`)
      (goto _label_2))))