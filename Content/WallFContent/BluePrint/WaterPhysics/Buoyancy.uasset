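; Buoyancy component that makes its owning actor float and drift in WaterBody actors.
; Owner overlap events track current water bodies, summing their flow and finding a surface height from their root Z.
; Each tick, static meshes tagged "Buoyancy" act as sample points, applying depth-scaled lift, linear drag and angular drag to the owner's static mesh.
; Water flow pushes the mesh while in water, even with buoyancy off.
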(event `self.ReceiveBeginPlay`
  (bind _returnvalue (`self.GetOwner`))
  ;[1 0.1269 0.1448] Begin Initialization
  (set `self.GravityZ` -980.0)
  (set `self.WaterFlowForce` (0.0 0.0 0.0))
  (bind _output_get (set `self.BuoList` (`Actor.GetComponentsByTag` _returnvalue "/Script/Engine.StaticMeshComponent" "Buoyancy")))
  (bind _output_get_2 (set `self.BuoAmount` (`KismetArrayLibrary.Array_Length` _output_get)))
  (if (<= _output_get_2 0)
    (set `self.Buoyancy` false))
  (add `Actor.OnActorBeginOverlap` _returnvalue (delegate `CustomEvent`))
  (add `Actor.OnActorEndOverlap` _returnvalue (delegate `CustomEvent_0`))
  (`KismetArrayLibrary.Array_Clear` (`self.WaterBodyList`))
  (set `self.WaterZTop` -100000000000000.0))

(event `CustomEvent`
  (params (OverlappedActor :type "Actor Object Reference") (OtherActor :type "Actor Object Reference"))
  (bind _aswater_body (cast `/Game/WallFContent/BluePrint/WaterPhysics/WaterBody` OtherActor))
  (`KismetArrayLibrary.Array_Add` (`self.WaterBodyList`) _aswater_body)
  (set `self.WaterFlowForce` (0.0 0.0 0.0) :!label _label)
  (for _array_element (`self.WaterBodyList`)
    (set `self.WaterFlowForce` (+ (`self.WaterFlowForce`) (`/Game/WallFContent/BluePrint/WaterPhysics/WaterBody.WaterFlow` _array_element)))
    (bind (_returnvalue_x _returnvalue_y _returnvalue_z) (`KismetMathLibrary.BreakVector` (`SceneComponent.K2_GetComponentLocation` (`Actor.RootComponent` _array_element))))
    (if (> _returnvalue_z (`self.WaterZTop`))
      (set `self.WaterZTop` _returnvalue_z)))
  (set `self.InWater` true))

(event `CustomEvent_0`
  (params (OverlappedActor :type "Actor Object Reference") (OtherActor :type "Actor Object Reference"))
  (bind _waterbodylist (`self.WaterBodyList`))
  (bind _aswater_body (cast `/Game/WallFContent/BluePrint/WaterPhysics/WaterBody` OtherActor))
  (`KismetArrayLibrary.Array_RemoveItem` _waterbodylist _aswater_body)
  (if (> (`KismetArrayLibrary.Array_Length` _waterbodylist) 0)
    (goto _label)
    (else
      (set `self.InWater` false)
      (set `self.WaterZTop` -100000000000000.0))))

(event `self.ReceiveTick`
  (params (DeltaSeconds :type "Float (single-precision)"))
  (bind _returnvalue (`GameplayStatics.GetWorldDeltaSeconds`))
  (bind _returnvalue_2 (`Actor.GetComponentByClass` (`self.GetOwner`) "/Script/Engine.StaticMeshComponent"))
  (if (and (`self.InWater`) (`self.Buoyancy`))
    ;[1 0.8122 0.4064] Init Variables & Loop
    (for _array_element (`self.BuoList`)
      (bind _returnvalue_3 (`SceneComponent.K2_GetComponentLocation` _array_element))
      (bind (_returnvalue_x _returnvalue_y _returnvalue_z) (`KismetMathLibrary.BreakVector` (+ _returnvalue_3 (0.0 0.0 0.0))))
      (bind _returnvalue_4 (* (`self.BuoAppliedForce`) (`KismetMathLibrary.FClamp` (`KismetMathLibrary.SafeDivide` (- (`self.WaterZTop`) _returnvalue_z) (`self.BuoDepth`)) 0.0 1000.0) 0.1))
      ;[0.3017 0.4763 1] Archimedes' principle
      (`PrimitiveComponent.AddForceAtLocation` _returnvalue_2 (`KismetMathLibrary.MakeVector` 0.0 0.0 (/ (* _returnvalue_4 (`KismetMathLibrary.Abs` (`self.GravityZ`))) (`self.BuoAmount`))) _returnvalue_3 "None")
      (bind (_returnvalue_x_2 _returnvalue_y_2 _returnvalue_z_2) (`KismetMathLibrary.BreakVector` (* _returnvalue _returnvalue_4 (`self.BuoDragForce`) (`KismetMathLibrary.NegateVector` (`SceneComponent.GetComponentVelocity` _returnvalue_2)))))
      ;[0.3992 0.3637 1] Fluid Drag Force
      (`PrimitiveComponent.AddForceAtLocation` _returnvalue_2 (`KismetMathLibrary.MakeVector` (/ _returnvalue_x_2 (`self.BuoAmount`)) (/ _returnvalue_y_2 (`self.BuoAmount`)) (/ _returnvalue_z_2 (`self.BuoAmount`))) _returnvalue_3 "None")
      (bind (_returnvalue_x_3 _returnvalue_y_3 _returnvalue_z_3) (`KismetMathLibrary.BreakVector` (* _returnvalue _returnvalue_4 (`self.BuoAngularDragForce`) (`KismetMathLibrary.NegateVector` (`PrimitiveComponent.GetPhysicsAngularVelocityInRadians` _returnvalue_2 "None")))))
      ;[0.4325 1 0.8735] Angular Drag Force
      (`PrimitiveComponent.AddTorqueInRadians` _returnvalue_2 (`KismetMathLibrary.MakeVector` (/ _returnvalue_x_3 (`self.BuoAmount`)) (/ _returnvalue_y_3 (`self.BuoAmount`)) (/ _returnvalue_z_3 (`self.BuoAmount`))) "None" true))
    (`PrimitiveComponent.AddForce` _returnvalue_2 (`self.WaterFlowForce`) "None" true :!label _label_2)
    (elif (`self.InWater`)
      (goto _label_2))))