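; BP_EndSplitTestOnly is a test-only trigger actor that ends the current speedrun split when the player enters it.
; On BeginPlay it caches the player's BP_Character and finds the level's BP_SpeedrunManager by class.
; When that character begins overlapping the BoxCollider, it calls EndCurrentSplit on the manager if the reference is valid.
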(event `self.ReceiveBeginPlay`
  (bind _asbp_character (cast `/Game/WallFContent/BluePrint/BP_Character` (`GameplayStatics.GetPlayerCharacter` 0)))
  (set `self.Character` _asbp_character)
  (bind _returnvalue (`GameplayStatics.GetActorOfClass` "/Game/WallFContent/BluePrint/Speedrun/BP_SpeedrunManager.BP_SpeedrunManager_C"))
  (set `self.SpeedrunManager` _returnvalue))

(event `self.BoxCollider.OnComponentBeginOverlap`
  (params (OverlappedComponent :type "PrimitiveComponent Object Reference") (OtherActor :type "Actor Object Reference") (OtherComp :type "PrimitiveComponent Object Reference") (OtherBodyIndex :type Integer) (bFromSweep :type Boolean) (SweepResult :type "HitResult Structure (by ref)"))
  (bind _speedrunmanager (`self.SpeedrunManager`))
  (if (== OtherActor (`self.Character`))
    (`/Engine/EditorBlueprintResources/StandardMacros.IsValid` _speedrunmanager
      (:`Is Valid`
        (`/Game/WallFContent/BluePrint/Speedrun/BP_SpeedrunManager.EndCurrentSplit` _speedrunmanager)))))

(fn `UserConstructionScript`)