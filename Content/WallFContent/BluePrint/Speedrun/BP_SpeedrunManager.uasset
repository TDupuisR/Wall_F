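; Speedrun manager that runs the overall timer and per-room split times and displays them on the game HUD.
; Tick accumulates time into the current split while the player is in a room, otherwise into a shared between-rooms (Intersalle) split.
; Split events start, pause, show or end splits, with ending showing a gap on the HUD.
; Saving writes the total and splits to BP_SaveGame as best time, without comparing against the previous one.
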(event `self.ReceiveBeginPlay`
  (bind _asbp_first_person_player_controller (cast `/Game/FirstPerson/Blueprints/BP_FirstPersonPlayerController` (`GameplayStatics.GetPlayerController` 0)))
  (set `self.Controller` _asbp_first_person_player_controller)
  (`self.LoadSpeedrunTime`)
  (bind _ashud_game (cast `/Game/WallFContent/BluePrint/HUD_Game` (`PlayerController.GetHUD` (`self.Controller`))))
  (set `self.HUD` _ashud_game))

(event `self.ReceiveTick`
  (params (DeltaSeconds :type "Float (single-precision)"))
  (bind _currentsplit (`self.CurrentSplit`))
  (bind _splittimes (`self.SplitTimes`))
  (bind _returnvalue (+ (`BlueprintMapLibrary.Map_Find` _splittimes _currentsplit) DeltaSeconds))
  (set `self.TimerTime` (+ (`self.TimerTime`) DeltaSeconds))
  (`/Game/WallFContent/Widgets/W_SpeedrunTimer.UpdateTimer` (`/Game/WallFContent/BluePrint/HUD_Game.Timer` (`self.HUD`)) (`self.TimerTime`))
  (if (`self.PlayerInRoom`)
    (`BlueprintMapLibrary.Map_Add` _splittimes _currentsplit _returnvalue)
    (`/Game/WallFContent/Widgets/W_SpeedrunTimer.UpdateSplit` (`/Game/WallFContent/BluePrint/HUD_Game.Timer` (`self.HUD`)) _currentsplit _returnvalue)
    (else
      (bind _output_get (set `self.IntersalleTime` (+ (`self.IntersalleTime`) DeltaSeconds)))
      (`/Game/WallFContent/Widgets/W_SpeedrunTimer.UpdateSplit` (`/Game/WallFContent/BluePrint/HUD_Game.Timer` (`self.HUD`)) "NewEnumerator1" _output_get)
      (`BlueprintMapLibrary.Map_Add` (`self.SplitTimes`) "NewEnumerator1" _output_get))))

(event `PauseCurrentSplit`
  (set `self.PlayerInRoom` false))

(event `StartSplit`
  (params (SplitName :type "/Game/WallFContent/BluePrint/Speedrun/E_SplitName Enum" :default "NewEnumerator0"))
  (`KismetSystemLibrary.PrintString` "start split")
  (set `self.PlayerInRoom` true)
  (set `self.CurrentSplit` SplitName))

(event `ShowSplit`
  (params (SplitName :type "/Game/WallFContent/BluePrint/Speedrun/E_SplitName Enum" :default "NewEnumerator0"))
  (`/Game/WallFContent/Widgets/W_SpeedrunTimer.ShowSplit` (`/Game/WallFContent/BluePrint/HUD_Game.Timer` (`self.HUD`)) SplitName))

(event `EndCurrentSplit`
  (bind _currentsplit (`self.CurrentSplit`))
  (`KismetSystemLibrary.PrintString` "end current split")
  (`/Game/WallFContent/Widgets/W_SpeedrunTimer.ShowGap` (`/Game/WallFContent/BluePrint/HUD_Game.Timer` (`self.HUD`)) _currentsplit (`BlueprintMapLibrary.Map_Find` (`self.SplitTimes`) _currentsplit)))

(event `LoadSpeedrunTime`
  (bind _returnvalue (`GameplayStatics.DoesSaveGameExist` (`self.SlotName`)))
  (if _returnvalue
    (bind _returnvalue_2 (`GameplayStatics.LoadGameFromSlot` (`self.SlotName`)))
    (bind _asbp_save_game (cast `/Game/WallFContent/BluePrint/Speedrun/BP_SaveGame` _returnvalue_2))
    (set `self.Save` _asbp_save_game)))

(event `SaveSpeedrunTime`
  (bind _timertime (`self.TimerTime`))
  (bind _splittimes (`self.SplitTimes`))
  (bind _value (`BlueprintMapLibrary.Map_Find` _splittimes "NewEnumerator0"))
  (bind _value_2 (`BlueprintMapLibrary.Map_Find` _splittimes "NewEnumerator4"))
  (bind _value_3 (`BlueprintMapLibrary.Map_Find` _splittimes "NewEnumerator1"))
  (bind _value_4 (`BlueprintMapLibrary.Map_Find` _splittimes "NewEnumerator2"))
  (bind _value_5 (`BlueprintMapLibrary.Map_Find` _splittimes "NewEnumerator3"))
  (bind _returnvalue (`GameplayStatics.DoesSaveGameExist` (`self.SlotName`)))
  (if _returnvalue
    (bind _returnvalue_2 (`GameplayStatics.LoadGameFromSlot` (`self.SlotName`)))
    (bind _asbp_save_game (cast `/Game/WallFContent/BluePrint/Speedrun/BP_SaveGame` _returnvalue_2))
    (set `/Game/WallFContent/BluePrint/Speedrun/BP_SaveGame.BestSpeedrunTime` _timertime _asbp_save_game)
    (set `/Game/WallFContent/BluePrint/Speedrun/BP_SaveGame.SplitTime_Tuto` _value _asbp_save_game)
    (set `/Game/WallFContent/BluePrint/Speedrun/BP_SaveGame.SplitTime_Intersalle` _value_3 _asbp_save_game)
    (set `/Game/WallFContent/BluePrint/Speedrun/BP_SaveGame.SplitTime_Ferdi` _value_4 _asbp_save_game)
    (set `/Game/WallFContent/BluePrint/Speedrun/BP_SaveGame.SplitTime_Paul` _value_5 _asbp_save_game)
    (set `/Game/WallFContent/BluePrint/Speedrun/BP_SaveGame.SplitTime_Daphne` _value_2 _asbp_save_game)
    (`GameplayStatics.SaveGameToSlot` _asbp_save_game (`self.SlotName`))
    (else
      (bind _returnvalue_3 (`GameplayStatics.CreateSaveGameObject` "/Game/WallFContent/BluePrint/Speedrun/BP_SaveGame.BP_SaveGame_C"))
      (set `/Game/WallFContent/BluePrint/Speedrun/BP_SaveGame.BestSpeedrunTime` _timertime _returnvalue_3)
      (set `/Game/WallFContent/BluePrint/Speedrun/BP_SaveGame.SplitTime_Tuto` _value _returnvalue_3)
      (set `/Game/WallFContent/BluePrint/Speedrun/BP_SaveGame.SplitTime_Intersalle` _value_3 _returnvalue_3)
      (set `/Game/WallFContent/BluePrint/Speedrun/BP_SaveGame.SplitTime_Ferdi` _value_4 _returnvalue_3)
      (set `/Game/WallFContent/BluePrint/Speedrun/BP_SaveGame.SplitTime_Paul` _value_5 _returnvalue_3)
      (set `/Game/WallFContent/BluePrint/Speedrun/BP_SaveGame.SplitTime_Daphne` _value_2 _returnvalue_3)
      (`GameplayStatics.SaveGameToSlot` _returnvalue_3 (`self.SlotName`)))))

(fn `GetSave`
  (returns (Save :type "/Game/WallFContent/BluePrint/Speedrun/BP_SaveGame Object Reference"))
  (bind _returnvalue (`GameplayStatics.DoesSaveGameExist` (`self.SlotName`)))
  (if _returnvalue
    (bind _returnvalue_2 (`GameplayStatics.LoadGameFromSlot` (`self.SlotName`)))
    (bind _asbp_save_game (cast `/Game/WallFContent/BluePrint/Speedrun/BP_SaveGame` _returnvalue_2))
    (return _asbp_save_game)
    (else
      (return null))))

(fn `UserConstructionScript`)