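; BP_EndSplitSpeedrun is a trigger volume that drives speedrun splits through the level's BP_SpeedrunManager, which it finds on BeginPlay.
; Entering its box collider starts the split named by SplitName.
; Leaving it ends the current split and shows each split listed in OnExitNewSplits.
; The overlap events do not filter the overlapping actor, and a BP_Character overlap check sits unconnected.
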(event `self.ReceiveBeginPlay`
  (bind _returnvalue (`GameplayStatics.GetActorOfClass` "/Game/WallFContent/BluePrint/Speedrun/BP_SpeedrunManager.BP_SpeedrunManager_C"))
  (set `self.SpeedrunManager` _returnvalue))

(event `self.BoxCollider.OnComponentBeginOverlap`
  (params (OverlappedComponent :type "PrimitiveComponent Object Reference") (OtherActor :type "Actor Object Reference") (OtherComp :type "PrimitiveComponent Object Reference") (OtherBodyIndex :type Integer) (bFromSweep :type Boolean) (SweepResult :type "HitResult Structure (by ref)"))
  (`/Game/WallFContent/BluePrint/Speedrun/BP_SpeedrunManager.StartSplit` (`self.SpeedrunManager`) (`self.SplitName`)))

(event `self.BoxCollider.OnComponentEndOverlap`
  (params (OverlappedComponent :type "PrimitiveComponent Object Reference") (OtherActor :type "Actor Object Reference") (OtherComp :type "PrimitiveComponent Object Reference") (OtherBodyIndex :type Integer))
  (bind _onexitnewsplits (`self.OnExitNewSplits`))
  (`/Game/WallFContent/BluePrint/Speedrun/BP_SpeedrunManager.EndCurrentSplit` (`self.SpeedrunManager`))
  (if (`KismetArrayLibrary.Array_IsNotEmpty` _onexitnewsplits)
    (for _array_element _onexitnewsplits
      (`/Game/WallFContent/BluePrint/Speedrun/BP_SpeedrunManager.ShowSplit` (`self.SpeedrunManager`) _array_element))))

(fn `UserConstructionScript`)