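; BP_SplitSpeedrun is a trigger volume that marks a named split for speedrun timing.
; On BeginPlay it finds and caches the BP_SpeedrunManager in the level.
; Its BoxCollider starts the split by SplitName on begin overlap and ends the current split on end overlap, without filtering the overlapping actor.
; An unconnected branch that would start the split when a BP_Character is already inside never runs.
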(event `self.ReceiveBeginPlay`
  (bind _returnvalue (`GameplayStatics.GetActorOfClass` "/Game/WallFContent/BluePrint/Speedrun/BP_SpeedrunManager.BP_SpeedrunManager_C"))
  (set `self.SpeedrunManager` _returnvalue))

(event `self.BoxCollider.OnComponentBeginOverlap`
  (params (OverlappedComponent :type "PrimitiveComponent Object Reference") (OtherActor :type "Actor Object Reference") (OtherComp :type "PrimitiveComponent Object Reference") (OtherBodyIndex :type Integer) (bFromSweep :type Boolean) (SweepResult :type "HitResult Structure (by ref)"))
  (`/Game/WallFContent/BluePrint/Speedrun/BP_SpeedrunManager.StartSplit` (`self.SpeedrunManager`) (`self.SplitName`)))

(event `self.BoxCollider.OnComponentEndOverlap`
  (params (OverlappedComponent :type "PrimitiveComponent Object Reference") (OtherActor :type "Actor Object Reference") (OtherComp :type "PrimitiveComponent Object Reference") (OtherBodyIndex :type Integer))
  (`/Game/WallFContent/BluePrint/Speedrun/BP_SpeedrunManager.EndCurrentSplit` (`self.SpeedrunManager`)))

(fn `UserConstructionScript`)