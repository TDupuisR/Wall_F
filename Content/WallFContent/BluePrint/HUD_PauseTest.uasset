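; HUD_PauseTest is a test Blueprint, named as a HUD, that puts the game straight into a paused state with the pause menu open.
; On BeginPlay it caches the BP_FirstPersonPlayerController, pauses the game, shows the mouse cursor and adds a W_PauseMenu widget to the viewport.
; It then stores the player's BP_Character, which this graph does not use further.
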(event `self.ReceiveBeginPlay`
  (bind _playercontroller (`self.PlayerController`))
  (bind _asbp_first_person_player_controller (cast `/Game/FirstPerson/Blueprints/BP_FirstPersonPlayerController` (`GameplayStatics.GetPlayerController` 0)))
  (set `self.PlayerController` _asbp_first_person_player_controller)
  (`GameplayStatics.SetGamePaused` true)
  (set `PlayerController.bShowMouseCursor` true _playercontroller)
  (bind _returnvalue (`|CreateWidget` "/Game/WallFContent/Widgets/W_PauseMenu.W_PauseMenu_C" _playercontroller))
  (bind _output_get (set `self.PauseMenu` _returnvalue))
  (`UserWidget.AddToViewport` _output_get 0)
  (bind _asbp_character (cast `/Game/WallFContent/BluePrint/BP_Character` (`GameplayStatics.GetPlayerCharacter` 0)))
  (set `self.Character` _asbp_character))

(fn `UserConstructionScript`)