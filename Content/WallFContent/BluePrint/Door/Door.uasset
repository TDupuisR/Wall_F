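; Door actor that toggles open and closed through a Call event, ignored while a transition is running.
; Transitions chain two MoveComponentTo animations around a delay: a front offset, then a side offset with rotation, reversed on closing, which also sets box collision to Block.
; Doors flagged open at BeginPlay snap by the front offset only.
; CheckID tests whether an asker's ID contains the door's non-empty ID.
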(event `self.ReceiveBeginPlay`
  (if (`self.IsOpened`)
    (`self.OpenDoorBeginning`)))

(event `OpenDoorWithTransition`
  (bind (_dooroffsetturn_x _dooroffsetturn_y _dooroffsetturn_z) (`KismetMathLibrary.BreakVector` (`self.DoorOffsetTurn`)))
  (bind _door (`self.Door`))
  (bind _door_2 (`self.Door`))
  (if (not (`self.IsOpened`))
    (set `self.IsRunning` true)
    (set `self.IsOpened` true)
    (`KismetSystemLibrary.PrintString` "open door with transition")
    (`KismetSystemLibrary.MoveComponentTo` _door (+ (`SceneComponent.RelativeLocation` _door) (`self.DoorOffsetFront`)) (`SceneComponent.RelativeRotation` _door) false false (`self.DoorTimeFront`))
    (`KismetSystemLibrary.Delay` (`self.TimeBeforeTurn`))
    (`KismetSystemLibrary.MoveComponentTo` _door_2 (+ (`SceneComponent.RelativeLocation` _door_2) (`self.DoorOffsetSide`)) (`KismetMathLibrary.MakeRotator` (+ (.roll (`SceneComponent.RelativeRotation` _door_2)) _dooroffsetturn_x) (+ (.pitch (`SceneComponent.RelativeRotation` _door_2)) _dooroffsetturn_y) (+ (.yaw (`SceneComponent.RelativeRotation` _door_2)) _dooroffsetturn_z)) false false (`self.DoorTimeTurn`))
    (set `self.IsRunning` false)))

(event `OpenDoorBeginning`
  (bind _door (`self.Door`))
  (`KismetSystemLibrary.PrintString` "open door beginning")
  (`SceneComponent.K2_SetRelativeLocation` _door (+ (`SceneComponent.RelativeLocation` _door) (`self.DoorOffsetFront`)) false false))

(event `CloseDoorWithTransition`
  (bind (_dooroffsetturn_x _dooroffsetturn_y _dooroffsetturn_z) (`KismetMathLibrary.BreakVector` (`self.DoorOffsetTurn`)))
  (bind _door (`self.Door`))
  (bind _door_2 (`self.Door`))
  (if (`self.IsOpened`)
    (set `self.IsRunning` true)
    (set `self.IsOpened` false)
    (`PrimitiveComponent.SetCollisionResponseToAllChannels` (`self.BoxCollision`) "ECR_Block")
    (`KismetSystemLibrary.PrintString` "close door with transition")
    (`KismetSystemLibrary.MoveComponentTo` _door_2 (- (`SceneComponent.RelativeLocation` _door_2) (`self.DoorOffsetSide`)) (`KismetMathLibrary.MakeRotator` (- (.roll (`SceneComponent.RelativeRotation` _door_2)) _dooroffsetturn_x) (- (.pitch (`SceneComponent.RelativeRotation` _door_2)) _dooroffsetturn_y) (- (.yaw (`SceneComponent.RelativeRotation` _door_2)) _dooroffsetturn_z)) false false (`self.DoorTimeTurn`))
    (`KismetSystemLibrary.Delay` (`self.TimeBeforeTurn`))
    (`KismetSystemLibrary.MoveComponentTo` _door (- (`SceneComponent.RelativeLocation` _door) (`self.DoorOffsetFront`)) (`SceneComponent.RelativeRotation` _door) false false (`self.DoorTimeFront`))
    (`PrimitiveComponent.SetCollisionResponseToAllChannels` (`self.BoxCollision`) "ECR_Block")
    (set `self.IsRunning` false)))

(event `/Game/WallFContent/BluePrint/EnvironmentInteractives/PressurePlate/I_Link.Call`
  (params (ActorID :type String) (IsActive :type Boolean))
  (if (`self.IsRunning`)
    _
    (elif (`self.IsOpened`)
      (`self.CloseDoorWithTransition`)
      (else
        (`self.OpenDoorWithTransition`)))))

(fn `CheckID`
  (params (AskerID :type String))
  (returns (IsSame :type Boolean))
  (bind _id (`self.ID`))
  (if (`KismetStringLibrary.IsEmpty` _id)
    (return false)
    (else
      (return (`KismetStringLibrary.Contains` AskerID _id)))))

(fn `UserConstructionScript`)