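; BP_LoadAndUnload is a trigger volume that streams levels in and out when the player character enters it.
; On BeginPlay it caches the player's BP_Character, and its BoxCollider overlap responds only to that actor.
; The overlap loads every level in LoadLevelNames, visible once loaded, then unloads those in UnloadLevelNames if that list is not empty, all without blocking.
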(event `self.ReceiveBeginPlay`
  (bind _asbp_character (cast `/Game/WallFContent/BluePrint/BP_Character` (`GameplayStatics.GetPlayerCharacter` 0)))
  (set `self.Character` _asbp_character))

(event `self.BoxCollider.OnComponentBeginOverlap`
  (params (OverlappedComponent :type "PrimitiveComponent Object Reference") (OtherActor :type "Actor Object Reference") (OtherComp :type "PrimitiveComponent Object Reference") (OtherBodyIndex :type Integer) (bFromSweep :type Boolean) (SweepResult :type "HitResult Structure (by ref)"))
  (bind _unloadlevelnames (`self.UnloadLevelNames`))
  (if (== OtherActor (`self.Character`))
    (if true
      (for _array_element (`self.LoadLevelNames`)
        (`GameplayStatics.LoadStreamLevel` _array_element true)))
    (if (`KismetArrayLibrary.Array_IsNotEmpty` _unloadlevelnames)
      (for _array_element_2 _unloadlevelnames
        (`GameplayStatics.UnloadStreamLevel` _array_element_2)))))

(fn `UserConstructionScript`)