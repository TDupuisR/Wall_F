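; BP_Cube is a physics cube the player moves and snaps onto other cubes to build attached assemblies.
; A sphere overlap collects nearby cubes, and Tick previews the nearest of six ghost sockets, which TryAttachCube uses to attach.
; Root and child searches let whole assemblies break apart with radial force, respawn at initial transforms after a delay, or toggle custom-depth rendering.
; A ground trace switches mass-scaled damping.
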(event `HideForRespawn`
  (params (Cube :type "/Game/WallFContent/BluePrint/Cube/BP_Cube Object Reference"))
  (bind _cube (`/Game/WallFContent/BluePrint/Cube/BP_Cube.Cube` Cube))
  (`PrimitiveComponent.SetCollisionResponseToAllChannels` _cube "ECR_Block")
  (`SceneComponent.SetVisibility` _cube false false))

(event `ShowAndChangePosRespawn`
  (params (Cube :type "/Game/WallFContent/BluePrint/Cube/BP_Cube Object Reference"))
  (bind _cube (`/Game/WallFContent/BluePrint/Cube/BP_Cube.Cube` Cube))
  (`PrimitiveComponent.SetCollisionResponseToAllChannels` _cube "ECR_Block")
  (`SceneComponent.K2_SetWorldLocation` _cube (`/Game/WallFContent/BluePrint/Cube/BP_Cube.InitialLocation` Cube) false false)
  (`SceneComponent.K2_SetWorldRotation` _cube (`/Game/WallFContent/BluePrint/Cube/BP_Cube.InitialRotation` Cube) false false)
  (`SceneComponent.SetVisibility` _cube true false))

(event `RespawnCube`
  (bind _root (`self.Root`))
  (bind _assembledcubechildren (`self.AssembledCubeChildren`))
  (`self.FindRoot`)
  (`self.GetCubeChildren` _root)
  (if (`self.IsMoving`)
    (`/Game/WallFContent/BluePrint/BP_Character.Drop` (`self.Character`)))
  (if (`KismetArrayLibrary.Array_IsNotEmpty` _assembledcubechildren)
    (for _array_element _assembledcubechildren
      (`self.DetachCubeWithoutForce` _array_element)
      (`self.HideForRespawn` _array_element))
    (`self.DetachCubeWithoutForce` _root)
    (`self.HideForRespawn` _root)
    (`KismetSystemLibrary.Delay` (`self.RespawnDelay`))
    (for _array_element_2 _assembledcubechildren
      (`self.ShowAndChangePosRespawn` _array_element_2)
      (`KismetArrayLibrary.Array_Clear` (`/Game/WallFContent/BluePrint/Cube/BP_Cube.AssembledCubeChildren` _array_element_2)))
    (`KismetArrayLibrary.Array_Clear` _assembledcubechildren)
    (`self.ShowAndChangePosRespawn` _root)
    (else
      (`self.HideForRespawn` self)
      (`KismetSystemLibrary.Delay` (`self.RespawnDelay`))
      (`self.ShowAndChangePosRespawn` self))))

(event `self.ReceiveBeginPlay`
  (bind _cube (`self.Cube`))
  ;[0.3005 0.2502 0.117] Begin Play - Hide Ghosts & Get Initial Location / Rotation
  (`self.HideCubeGhosts`)
  (set `self.InitialLocation` (`SceneComponent.K2_GetComponentLocation` _cube))
  (set `self.InitialRotation` (`SceneComponent.K2_GetComponentRotation` _cube))
  (bind _asbp_character (cast `/Game/WallFContent/BluePrint/BP_Character` (`GameplayStatics.GetPlayerCharacter` 0)))
  (set `self.Character` _asbp_character))

(event `GetNearestParent`
  (bind _tempparentsmindistances (`self.TempParentsMinDistances`))
  ;[0.1221 0.0999 0.3005] Get Nearest Parent (Multiple in Overlap)
  (if (`KismetArrayLibrary.Array_IsNotEmpty` _tempparentsmindistances)
    (`KismetArrayLibrary.Array_Clear` _tempparentsmindistances))
  (for _array_element (`self.ParentsInCollider`)
    (`self.GetTempMinDistanceParentSockets` _array_element))
  (`self.SetNearestParent` (`|GetArrayItem` (`self.ParentsInCollider`) (`KismetMathLibrary.MinOfFloatArray` (`self.TempParentsMinDistances`)))))

(event `self.ReceiveTick`
  (params (DeltaSeconds :type "Float (single-precision)"))
  ;[0.3005 0.2502 0.117] Event Tick - Show Ghost
  ;;[0.3719 0.1588 0.03215] Grounded Behaviour
  (bind _grounded (`self.IsGrounded` (`self.Cube`)))
  (`self.SetDamping` _grounded)
  (if (`KismetArrayLibrary.Array_IsNotEmpty` (`self.ParentsInCollider`))
    (`self.GetNearestParent`)
    (`/Engine/EditorBlueprintResources/StandardMacros.IsValid` (`self.NearestParentCube`)
      (:`Is Valid`
        (`self.CheckCanAttachCube`)
        (if (`self.CanAttachCube`)
          (`self.ShowNearestParentCubeGhost`))))))

(event `TryAttachCube`
  ;[0.3 0.1394 0.03821] Check & Attach Cube
  (if (`KismetArrayLibrary.Array_IsNotEmpty` (`self.ParentsInCollider`))
    (`self.GetNearestParent`)
    (`/Engine/EditorBlueprintResources/StandardMacros.IsValid` (`self.NearestParentCube`)
      (:`Is Valid`
        (`self.CheckCanAttachCube`)
        (if (`self.CanAttachCube`)
          (`self.AttachToNearestCube`))))))

(event `SetNearestParent`
  (params (Parent :type "/Game/WallFContent/BluePrint/Cube/BP_Cube Object Reference"))
  (bind _nearestparentcube (`self.NearestParentCube`))
  ;[0.1221 0.0999 0.3005] Set Nearest Parent
  (`/Engine/EditorBlueprintResources/StandardMacros.IsValid` _nearestparentcube
    (:`Is Valid`
      (if (!= Parent _nearestparentcube)
        (`self.HideAllParentGhosts`)
        (bind _output_get (set `self.NearestParentCube` Parent :!label _label))
        (set `self.NearestParentCubeRoot` (`Actor.RootComponent` _output_get))))
    (:`Is Not Valid`
      (goto _label))))

(event `self.SphereCollider.OnComponentBeginOverlap`
  (params (OverlappedComponent :type "PrimitiveComponent Object Reference") (OtherActor :type "Actor Object Reference") (OtherComp :type "PrimitiveComponent Object Reference") (OtherBodyIndex :type Integer) (bFromSweep :type Boolean) (SweepResult :type "HitResult Structure (by ref)"))
  ;[0.1798 0.3 0.1135] Begin Overlap - Add Parent
  (bind _asbp_cube (cast `/Game/WallFContent/BluePrint/Cube/BP_Cube` OtherActor))
  (if (!= _asbp_cube self)
    (`KismetArrayLibrary.Array_AddUnique` (`self.ParentsInCollider`) _asbp_cube)))

(event `HideCubeGhosts`
  ;[0.3005 0.2502 0.117] Show / Hide Ghosts
  (for _array_element (`self.Ghosts`)
    (`SceneComponent.SetVisibility` _array_element false false)))

(event `HideAllParentGhosts`
  (bind _nearestparentcube (`self.NearestParentCube`))
  ;[0.3005 0.2502 0.117] Show / Hide Ghosts
  (`/Engine/EditorBlueprintResources/StandardMacros.IsValid` _nearestparentcube
    (:`Is Valid`
      (for _array_element (`/Game/WallFContent/BluePrint/Cube/BP_Cube.Ghosts` _nearestparentcube)
        (`SceneComponent.SetVisibility` _array_element false false)))))

(event `self.SphereCollider.OnComponentEndOverlap`
  (params (OverlappedComponent :type "PrimitiveComponent Object Reference") (OtherActor :type "Actor Object Reference") (OtherComp :type "PrimitiveComponent Object Reference") (OtherBodyIndex :type Integer))
  ;[0.1798 0.3 0.1135] End Overlap - Remove Parent + Hide Ghosts
  (bind _asbp_cube (cast `/Game/WallFContent/BluePrint/Cube/BP_Cube` OtherActor))
  (`self.HideAllParentGhosts`)
  (`KismetArrayLibrary.Array_RemoveItem` (`self.ParentsInCollider`) _asbp_cube))

(event `ShowNearestParentCubeGhost`
  ;[0.3005 0.2502 0.117] Show / Hide Ghosts
  (`self.GetParentNearestSocket`)
  (`self.HideAllParentGhosts`)
  (`SceneComponent.SetVisibility` (`|GetArrayItem` (`/Game/WallFContent/BluePrint/Cube/BP_Cube.Ghosts` (`self.NearestParentCube`)) (`self.NearestParentGhostIndex`)) true false))

(event `GetDistancesFromEachParentSocket`
  (params (Parent :type "/Game/WallFContent/BluePrint/Cube/BP_Cube Object Reference"))
  ;[0.3005 0.0999 0.2462] Get Distances From Each Parent Socket
  (for _array_element (`/Game/WallFContent/BluePrint/Cube/BP_Cube.Ghosts` Parent)
    (`KismetArrayLibrary.Array_Add` (`self.NearestParentGhostsDistances`) (`KismetMathLibrary.Vector_Distance` (`SceneComponent.K2_GetComponentLocation` _array_element) (`SceneComponent.K2_GetComponentLocation` (`self.Cube`))))))

(event `GetTempMinDistanceParentSockets`
  (params (Parent :type "/Game/WallFContent/BluePrint/Cube/BP_Cube Object Reference"))
  (bind _tempparentghostsdistances (`self.TempParentGhostsDistances`))
  ;[0.3005 0.0999 0.2462] Get Temp Min Distances From A Parent Sockets
  (if (`KismetArrayLibrary.Array_IsNotEmpty` _tempparentghostsdistances)
    (`KismetArrayLibrary.Array_Clear` _tempparentghostsdistances))
  (for _array_element (`/Game/WallFContent/BluePrint/Cube/BP_Cube.Ghosts` Parent)
    (`KismetArrayLibrary.Array_Add` (`self.TempParentGhostsDistances`) (`KismetMathLibrary.Vector_Distance` (`SceneComponent.RelativeLocation` _array_element) (`SceneComponent.K2_GetComponentLocation` (`self.Cube`)))))
  (`KismetArrayLibrary.Array_Add` (`self.TempParentsMinDistances`) (`.MinValue` (`KismetMathLibrary.MinOfFloatArray` (`self.TempParentGhostsDistances`)))))

(event `AttachToNearestCube`
  (bind _socketsbool (`self.SocketsBool`))
  (bind _cube (`self.Cube`))
  (bind _nearestparentghostindex (`self.NearestParentGhostIndex`))
  (bind _socketsbool_2 (`/Game/WallFContent/BluePrint/Cube/BP_Cube.SocketsBool` (`self.NearestParentCube`)))
  (bind _returnvalue_location (`KismetMathLibrary.BreakTransform` (`KismetMathLibrary.MakeRelativeTransform` (`SceneComponent.K2_GetComponentToWorld` (`|GetArrayItem` (`self.Ghosts`) (`self.NearestParentGhostIndex`))) (`SceneComponent.K2_GetComponentToWorld` _cube))))
  (`self.CheckCanAttachCube`)
  (if (`self.CanAttachCube`)
    ;[0.09978 0.291 0.3] Moving Cube : 0 parent & children
    (if (== (`KismetArrayLibrary.Array_Length` (`self.GetAttachedActors` true)) 0)
      (`/Engine/EditorBlueprintResources/StandardMacros.IsValid` (`self.GetParentActor`)
        (:`Is Not Valid`
          (`self.GetParentNearestSocket`)
          (if (not (== (`|GetArrayItem` _socketsbool_2 (`self.NearestParentGhostIndex`)) true))
            (`KismetArrayLibrary.Array_Set` _socketsbool_2 _nearestparentghostindex true)
            (`KismetSystemLibrary.LogString` (`KismetStringLibrary.Conv_IntToString` _nearestparentghostindex))
            (switch `int` (`self.NearestParentGhostIndex`)
              (:`0`
                (`KismetArrayLibrary.Array_Set` _socketsbool 2 true))
              (:`1`
                (`KismetArrayLibrary.Array_Set` _socketsbool 3 true))
              (:`2`
                (`KismetArrayLibrary.Array_Set` _socketsbool 0 true))
              (:`3`
                (`KismetArrayLibrary.Array_Set` _socketsbool 1 true))
              (:`4`
                (`KismetArrayLibrary.Array_Set` _socketsbool 5 true))
              (:`5`
                (`KismetArrayLibrary.Array_Set` _socketsbool 4 true)))
            (`KismetSystemLibrary.LogString` (`KismetStringLibrary.Concat_StrStr` "set parent : " (`KismetSystemLibrary.GetDisplayName` (`self.NearestParentCubeRoot`)) ", at cube : " (`KismetSystemLibrary.GetDisplayName` (`self.Cube`))))
            (`self.K2_AttachToComponent` (`self.NearestParentCubeRoot`) "None" "KeepWorld" "SnapToTarget" "KeepWorld")
            (`KismetSystemLibrary.MoveComponentTo` _cube _returnvalue_location)
            (set `self.IsMoving` false)
            (`self.HideAllParentGhosts`)))))))

(event `GetParentNearestSocket`
  (bind _nearestparentcube (`self.NearestParentCube`))
  (bind _indexofminvalue (`KismetMathLibrary.MinOfFloatArray` (`self.NearestParentGhostsDistances`)))
  ;[0.3005 0.0999 0.2462] Get Parent Nearest Socket
  (`self.GetDistancesFromEachParentSocket` _nearestparentcube)
  (set `self.NearestParentGhostIndex` _indexofminvalue)
  (set `self.NearestParentGhostLocation` (`SceneComponent.RelativeLocation` (`|GetArrayItem` (`/Game/WallFContent/BluePrint/Cube/BP_Cube.Ghosts` _nearestparentcube) _indexofminvalue))))

(event `CheckCanAttachCube`
  (bind _nearestparentcube (`self.NearestParentCube`))
  (bind _nearestparentghostsdistances (`self.NearestParentGhostsDistances`))
  ;[0.1219 0.2069 0.3] Check Can Attach Cube
  (set `self.CanAttachCube` false)
  (if (`KismetArrayLibrary.Array_IsNotEmpty` _nearestparentghostsdistances)
    (`KismetArrayLibrary.Array_Clear` _nearestparentghostsdistances))
  (if (`self.IsMoving`)
    (if (`/Game/WallFContent/BluePrint/Cube/BP_Cube.IsMoving` _nearestparentcube)
      _
      (elif (!= _nearestparentcube self)
        (set `self.CanAttachCube` true)))))

(event `DetachAllAssembledCubesWithForce`
  (bind _root (`self.Root`))
  (bind _assembledcubechildren (`self.AssembledCubeChildren`))
  (bind _assembledcubechildren_2 (`self.AssembledCubeChildren`))
  ;[0.3005 0.04374 0.05286] Detach All Assembled Cubes
  (`self.FindRoot`)
  (if (`KismetArrayLibrary.Array_IsNotEmpty` _assembledcubechildren_2)
    (`KismetArrayLibrary.Array_Clear` _assembledcubechildren_2))
  (`self.GetCubeChildren` _root)
  (if (`KismetArrayLibrary.Array_IsNotEmpty` _assembledcubechildren)
    (for _array_element _assembledcubechildren
      (`self.DetachCubeWithForce` _array_element))
    (`self.DetachCubeWithForce` _root)
    (for _array_element_2 _assembledcubechildren
      (`KismetArrayLibrary.Array_Clear` (`/Game/WallFContent/BluePrint/Cube/BP_Cube.AssembledCubeChildren` _array_element_2)))
    (`KismetArrayLibrary.Array_Clear` _assembledcubechildren)))

(event `FindRoot`
  (bind _returnvalue (`self.GetAttachParentActor` (`self.Root`)))
  ;[0.3005 0.04374 0.05286] Find Cube Root
  (bind _asbp_cube (cast `/Game/WallFContent/BluePrint/Cube/BP_Cube` (`self.GetAttachParentActor` self))
    (:`then`
      (`/Engine/EditorBlueprintResources/StandardMacros.IsValid` _asbp_cube
        (:`Is Valid`
          (set `self.Root` _asbp_cube)
          (set `self.FoundParent` true)
          (while (`self.FoundParent`)
            (`/Engine/EditorBlueprintResources/StandardMacros.IsValid` _returnvalue
              (:`Is Valid`
                (bind _asbp_cube_2 (cast `/Game/WallFContent/BluePrint/Cube/BP_Cube` _returnvalue)
                  (:`then`
                    (set `self.Root` _asbp_cube_2))
                  (:`CastFailed`
                    (set `self.FoundParent` false :!label _label_2))))
              (:`Is Not Valid`
                (goto _label_2)))))
        (:`Is Not Valid`
          (set `self.Root` self :!label _label_3))))
    (:`CastFailed`
      (goto _label_3))))

(event `GetCubeChildren`
  (params (Cube :type "/Game/WallFContent/BluePrint/Cube/BP_Cube Object Reference"))
  (bind _outactors (`self.GetAttachedActors` Cube true true))
  ;[0.3005 0.04374 0.05286] Get All Cube Chidren From Root
  (if (`KismetArrayLibrary.Array_IsNotEmpty` _outactors)
    (for _array_element _outactors
      (bind _asbp_cube (cast `/Game/WallFContent/BluePrint/Cube/BP_Cube` _array_element))
      (if (!= _array_element (`self.Root`))
        (`KismetArrayLibrary.Array_AddUnique` (`self.AssembledCubeChildren`) _asbp_cube)))))

(event `DetachCubeWithoutForce`
  (params (Cube :type "/Game/WallFContent/BluePrint/Cube/BP_Cube Object Reference"))
  (bind _socketsbool (`/Game/WallFContent/BluePrint/Cube/BP_Cube.SocketsBool` Cube))
  ;[0.3005 0.04374 0.05286] Detach Cube Without Force
  (`self.K2_DetachFromActor` Cube "KeepWorld" "KeepWorld" "KeepWorld")
  (set `/Game/WallFContent/BluePrint/Cube/BP_Cube.IsMoving` false Cube)
  (for (_ _array_index) _socketsbool
    (`KismetArrayLibrary.Array_Set` _socketsbool _array_index)))

(event `DetachEffectOnCube`
  (params (Cube :type "/Game/WallFContent/BluePrint/Cube/BP_Cube Object Reference"))
  (bind _cube (`/Game/WallFContent/BluePrint/Cube/BP_Cube.Cube` Cube))
  ;[0.3005 0.04374 0.05286] Detach Effect On Cube
  (`PrimitiveComponent.AddRadialForce` _cube (`SceneComponent.K2_GetComponentLocation` _cube) (`self.DetachRadius`) (`self.DetachForce`) "RIF_Constant" false))

(event `DetachCubeWithForce`
  (params (Cube :type "/Game/WallFContent/BluePrint/Cube/BP_Cube Object Reference"))
  ;[0.3005 0.04374 0.05286] Detach Cube With Force
  (`self.DetachCubeWithoutForce` Cube)
  (`self.DetachEffectOnCube` Cube))

(event `/Game/WallFContent/BluePrint/I_Interactable.SetMaterial`
  (params (Active :type Boolean))
  (bind _returnvalue (`KismetArrayLibrary.Array_Length` (`self.AssembledCubeChildren`)))
  ;[1 1 1] Set Material PostProcess
  (`self.FindRoot`)
  (`self.GetCubeChildren` (`self.Root`))
  (if (> _returnvalue 0)
    _
    (else
      _))
  (`PrimitiveComponent.SetRenderCustomDepth` (`/Game/WallFContent/BluePrint/Cube/BP_Cube.Cube` (`self.Root`)) Active)
  (for _ (range _returnvalue)
    ;;[0 0 0] SetMaterial on all children
    (`PrimitiveComponent.SetRenderCustomDepth` (`/Game/WallFContent/BluePrint/Cube/BP_Cube.Cube` (`|GetArrayItem` (`self.AssembledCubeChildren`))) Active)))

(fn `DoesPostProcessActive`
  (returns (isActive :type Boolean))
  (return (`PrimitiveComponent.bRenderCustomDepth` (`self.Cube`))))

(fn `IsGrounded`
  (params (SceneComp :type "SceneComponent Object Reference"))
  (returns (Grounded :type Boolean))
  (bind _returnvalue (`SceneComponent.K2_GetComponentLocation` SceneComp))
  (bind (_outhit _returnvalue_2) (`KismetSystemLibrary.LineTraceSingle` :`Start` _returnvalue :`End` (`KismetMathLibrary.MakeVector` (.x _returnvalue) (.y _returnvalue) (+ (.z _returnvalue) (`self.ProxyDistance`))) :`TraceChannel` "TraceTypeQuery1" :`DrawDebugType` "Persistent"))
  (return _returnvalue_2))

(fn `SetDamping`
  (params (Grounded :type Boolean))
  (bind _cube (`self.Cube`))
  (bind _cube_2 (`self.Cube`))
  (bind _returnvalue (`PrimitiveComponent.GetMass` _cube_2))
  (if Grounded
    (`PrimitiveComponent.SetLinearDamping` _cube_2 (* _returnvalue (`self.LinearDamping`)))
    (`PrimitiveComponent.SetAngularDamping` _cube_2 (* _returnvalue (`self.AngularDamping`)))
    (else
      (`PrimitiveComponent.SetLinearDamping` _cube 0.01)
      (`PrimitiveComponent.SetAngularDamping` _cube 0.0))))

(fn `UserConstructionScript`
  (bind _ghosts (`self.Ghosts`))
  (bind _socketsbool (`self.SocketsBool`))
  (bind _parentsincollider (`self.ParentsInCollider`))
  (for (_ _array_index) _socketsbool
    (`KismetArrayLibrary.Array_Set` _socketsbool _array_index))
  ;[0.3 0.3 0.3] Set Ghosts
  (if (`KismetArrayLibrary.Array_IsNotEmpty` _ghosts)
    (`KismetArrayLibrary.Array_Clear` _ghosts))
  (`KismetArrayLibrary.Array_Add` _ghosts (`self.Ghost_0`))
  (`KismetArrayLibrary.Array_Add` _ghosts (`self.Ghost_1`))
  (`KismetArrayLibrary.Array_Add` _ghosts (`self.Ghost_2`))
  (`KismetArrayLibrary.Array_Add` _ghosts (`self.Ghost_3`))
  (`KismetArrayLibrary.Array_Add` _ghosts (`self.Ghost_4`))
  (`KismetArrayLibrary.Array_Add` _ghosts (`self.Ghost_5`))
  ;[1 1 1] Clear Parents In Collider
  (if (`KismetArrayLibrary.Array_IsNotEmpty` _parentsincollider)
    (`KismetArrayLibrary.Array_Clear` _parentsincollider)))