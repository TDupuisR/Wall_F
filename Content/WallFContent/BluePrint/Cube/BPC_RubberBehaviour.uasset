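; Component that gives its owning cube actor rubber behaviour: tyre-block look, rubber sound, buoyancy and bounce.
; On BeginPlay, a single "Cube"-tagged mesh triggers overrides of mass, mesh, materials, BPC_Buoyancy tuning and physical material, plus hit binding; otherwise only the sound is set.
; Hits against non-I_Cube actors above a vertical speed threshold add capped upward acceleration scaled by that speed.
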(event `self.ReceiveBeginPlay`
  (bind _returnvalue (`self.GetOwner`))
  (bind _returnvalue_2 (`Actor.GetComponentByClass` _returnvalue "/Script/Engine.AudioComponent"))
  (bind _returnvalue_3 (`Actor.GetComponentByClass` _returnvalue "/Script/Engine.PrimitiveComponent"))
  (bind _returnvalue_4 (`Actor.GetComponentByClass` _returnvalue "/Game/WallFContent/BluePrint/WaterPhysics/BPC_Buoyancy.BPC_Buoyancy_C"))
  (bind _returnvalue_5 (`Actor.GetComponentsByTag` _returnvalue "/Script/Engine.StaticMeshComponent" "Cube"))
  (bind _output (`|GetArrayItem` _returnvalue_5))
  (if (== (`KismetArrayLibrary.Array_Length` _returnvalue_5) 1)
    (`PrimitiveComponent.SetMassOverrideInKg` _output "None" 150.0 true)
    (`StaticMeshComponent.SetStaticMesh` _output "/Game/WallFContent/ART/01_Mesh/Pneu_Block.Pneu_Block")
    (for (_array_element _array_index) (`self.Materials`)
      (`PrimitiveComponent.SetMaterial` _output _array_index _array_element))
    (set `/Game/WallFContent/BluePrint/WaterPhysics/BPC_Buoyancy.BuoDepth` 1.2 _returnvalue_4)
    (set `/Game/WallFContent/BluePrint/WaterPhysics/BPC_Buoyancy.BuoDragForce` 100.0 _returnvalue_4)
    (set `/Game/WallFContent/BluePrint/WaterPhysics/BPC_Buoyancy.BuoAppliedForce` 20.0 _returnvalue_4)
    (set `/Game/WallFContent/BluePrint/WaterPhysics/BPC_Buoyancy.BuoAngularDragForce` 0.5 _returnvalue_4)
    (`PrimitiveComponent.SetPhysMaterialOverride` _returnvalue_3 "/Game/WallFContent/BluePrint/Cube/PhysicsMaterial/PM_Bounce.PM_Bounce")
    (`AudioComponent.SetSound` _returnvalue_2 "/Game/WallFContent/Sounds/AudioRubber.AudioRubber")
    (add `PrimitiveComponent.OnComponentHit` _returnvalue_3 (delegate `CE_Bounce`))
    (else
      (`AudioComponent.SetSound` _returnvalue_2 "/Game/WallFContent/Sounds/AudioRubber.AudioRubber"))))

(event `CE_Bounce`
  (params (HitComponent :type "PrimitiveComponent Object Reference") (OtherActor :type "Actor Object Reference") (OtherComp :type "PrimitiveComponent Object Reference") (NormalImpulse :type "Vector Structure") (Hit :type "HitResult Structure (by ref)"))
  (bind _returnvalue (`Actor.GetComponentByClass` (`self.GetOwner`) "/Script/Engine.PrimitiveComponent"))
  (if (not (`KismetSystemLibrary.DoesImplementInterface` OtherActor "/Game/WallFContent/BluePrint/Cube/I_Cube.I_Cube_C"))
    (bind _returnvalue_2 (`PrimitiveComponent.GetPhysicsLinearVelocity` _returnvalue "None"))
    (bind _returnvalue_3 (`KismetMathLibrary.Abs` (.z _returnvalue_2)))
    (if (> _returnvalue_3 50.0)
      (bind _returnvalue_4 (* (/ _returnvalue_3 4.0) 200.0))
      (if (> _returnvalue_4 8001.0)
        (`PrimitiveComponent.AddForce` _returnvalue (0.0 0.0 8000.0) "None" true)
        (else
          (`PrimitiveComponent.AddForce` _returnvalue (`KismetMathLibrary.MakeVector` 0.0 0.0 _returnvalue_4) "None" true))))))