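; Actor component that gives a cube actor metal physical behaviour, tuning its mass and buoyancy.
; On BeginPlay it finds the owner's single static mesh tagged "Cube", overrides it to a heavy mass, and sets depth, drag and force values on the sibling BPC_Buoyancy component.
; It logs an error if zero or several tagged meshes are found.
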(event `self.ReceiveBeginPlay`
  (bind _returnvalue (`self.GetOwner`))
  (bind _returnvalue_2 (`Actor.GetComponentByClass` _returnvalue "/Game/WallFContent/BluePrint/WaterPhysics/BPC_Buoyancy.BPC_Buoyancy_C"))
  (bind _returnvalue_3 (`Actor.GetComponentsByTag` _returnvalue "/Script/Engine.StaticMeshComponent" "Cube"))
  (if (== (`KismetArrayLibrary.Array_Length` _returnvalue_3) 1)
    (`PrimitiveComponent.SetMassOverrideInKg` (`|GetArrayItem` _returnvalue_3) "None" 500.0 true)
    (set `/Game/WallFContent/BluePrint/WaterPhysics/BPC_Buoyancy.BuoDepth` 1.0 _returnvalue_2)
    (set `/Game/WallFContent/BluePrint/WaterPhysics/BPC_Buoyancy.BuoDragForce` 100.0 _returnvalue_2)
    (set `/Game/WallFContent/BluePrint/WaterPhysics/BPC_Buoyancy.BuoAppliedForce` 20.0 _returnvalue_2)
    (set `/Game/WallFContent/BluePrint/WaterPhysics/BPC_Buoyancy.BuoAngularDragForce` 2.0 _returnvalue_2)
    (else
      (`KismetSystemLibrary.LogString` (`KismetStringLibrary.Concat_StrStr` (`KismetSystemLibrary.GetObjectName` _returnvalue) ": Error no or too many Cubes detected, check StaticMeshs Tags")))))