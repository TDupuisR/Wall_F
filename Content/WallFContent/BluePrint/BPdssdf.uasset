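; BPdssdf is a Blueprint that switches the physics damping of its Cube according to a ground check.
; Each Tick runs the check and passes the result to SetDamping.
; Grounded line-traces on the Visibility channel along Z by ProxyDistance, with persistent debug drawing.
; When grounded, linear and angular damping scale with the Cube's mass; otherwise they drop to near zero.
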(event `self.ReceiveTick`
  (params (DeltaSeconds :type "Float (single-precision)"))
  (bind _grounded (`/Game/WallFContent/BluePrint/I_Interactable.IsGrounded` (`self.Cube`)))
  (`self.Set Damping` _grounded))

(fn `Grounded`
  (params (Scene :type "SceneComponent Object Reference"))
  (returns (Grounded :type Boolean))
  (bind _returnvalue (`SceneComponent.K2_GetComponentLocation` Scene))
  (bind (_outhit _returnvalue_2) (`KismetSystemLibrary.LineTraceSingle` :`Start` _returnvalue :`End` (`KismetMathLibrary.MakeVector` (.x _returnvalue) (.y _returnvalue) (+ (.z _returnvalue) (`self.ProxyDistance`))) :`TraceChannel` "TraceTypeQuery1" :`DrawDebugType` "Persistent"))
  (return _returnvalue_2))

(fn `Set Damping`
  (params (Grounded :type Boolean))
  (bind _cube (`self.Cube`))
  (bind _cube_2 (`self.Cube`))
  (bind _returnvalue (`PrimitiveComponent.GetMass` _cube_2))
  (if Grounded
    (`PrimitiveComponent.SetLinearDamping` _cube_2 (* _returnvalue (`self.LinearDamping`)))
    (`PrimitiveComponent.SetAngularDamping` _cube_2 (* _returnvalue (`self.AngularDamping`)))
    (else
      (`PrimitiveComponent.SetLinearDamping` _cube 0.01)
      (`PrimitiveComponent.SetAngularDamping` _cube 0.0))))

(fn `UserConstructionScript`)