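; Physics shelf prop that plays a bounce sound on impact, with pitch scaled by its speed.
; Tick caches the shelf's location and line-traces for ground, setting WasPlayed to mute hits while grounded.
; On hit, the audio triggers once until the next Tick reset, if velocity and both horizontal and vertical displacement pass thresholds.
; SetMaterial toggles custom depth rendering, while DoesPostProcessActive always returns false.
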(event `self.ReceiveTick`
  (params (DeltaSeconds :type "Float (single-precision)"))
  (bind _shelf (`self.Shelf`))
  (set `self.LastFrameLocation` (`SceneComponent.K2_GetComponentLocation` _shelf))
  (bind _grounded (`self.IsGrounded` _shelf))
  (set `self.WasPlayed` _grounded))

(event `self.Shelf.OnComponentHit`
  (params (HitComponent :type "PrimitiveComponent Object Reference") (OtherActor :type "Actor Object Reference") (OtherComp :type "PrimitiveComponent Object Reference") (NormalImpulse :type "Vector Structure") (Hit :type "HitResult Structure (by ref)"))
  (bind _shelf (`self.Shelf`))
  (bind _audio (`self.Audio`))
  (if (not (`self.WasPlayed`))
    (set `self.WasPlayed` true)
    (bind _returnvalue (`PrimitiveComponent.GetPhysicsLinearVelocity` _shelf "None"))
    (bind _returnvalue_2 (`KismetMathLibrary.VSize` _returnvalue))
    (if (and (> _returnvalue_2 50.0) (or (> (`KismetMathLibrary.Abs` (.x (- (`SceneComponent.K2_GetComponentLocation` _shelf) (`self.LastFrameLocation`)))) 1.0) (> (`KismetMathLibrary.Abs` (.y (- (`SceneComponent.K2_GetComponentLocation` _shelf) (`self.LastFrameLocation`)))) 1.0)) (> (`KismetMathLibrary.Abs` (.z (- (`SceneComponent.K2_GetComponentLocation` _shelf) (`self.LastFrameLocation`)))) 1.0))
      (`AudioComponent.SetFloatParameter` _audio "Pitch" (/ _returnvalue_2 100.0))
      (`AudioParameterControllerInterface.SetTriggerParameter` _audio "Bouncing"))))

(event `self.SetMaterial`
  (params (Active :type Boolean))
  (`PrimitiveComponent.SetRenderCustomDepth` (`self.Shelf`) Active))

(fn `DoesPostProcessActive`
  (returns (isActive :type Boolean))
  (return false))

(fn `IsGrounded`
  (params (SceneComp :type "SceneComponent Object Reference"))
  (returns (Grounded :type Boolean) (Beam :type "/Game/WallFContent/BluePrint/EnvironmentInteractives/BP_RotatingBeam Object Reference"))
  (bind _returnvalue (`SceneComponent.K2_GetComponentLocation` SceneComp))
  (bind (_outhit _returnvalue_2) (`KismetSystemLibrary.LineTraceSingle` (+ _returnvalue (0.0 0.0 10.0)) (`KismetMathLibrary.MakeVector` (.x _returnvalue) (.y _returnvalue) (+ (.z _returnvalue) (`self.Proxy Distance`))) "TraceTypeQuery3" true))
  (return _returnvalue_2 null))

(fn `UserConstructionScript`)