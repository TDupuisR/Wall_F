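; Physics actor Blueprint that adjusts the linear and angular damping of its Cube component every tick.
; Tick passes an IsGrounded result to Setdamping, which scales configurable damping values by the cube's mass.
; The branch condition is fixed to true, so the grounded result is ignored and the low-damping fallback never applies.
; A debug line trace using ProxyDistance is left unconnected and never runs.
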(event `self.ReceiveTick`
  (params (DeltaSeconds :type "Float (single-precision)"))
  (bind _grounded (`/Game/WallFContent/BluePrint/I_Interactable.IsGrounded` (`self.Cube`)))
  (`self.setdamping` _grounded))

(fn `setdamping`
  (params (`>Grounded` :type Boolean))
  (bind _cube (`self.Cube`))
  (bind _cube_2 (`self.Cube`))
  (bind _returnvalue (`PrimitiveComponent.GetMass` _cube_2))
  (if true
    (`PrimitiveComponent.SetLinearDamping` _cube_2 (* _returnvalue (`self.LinearDamping`)))
    (`PrimitiveComponent.SetAngularDamping` _cube_2 (* _returnvalue (`self.AngularDamping`)))
    (else
      (`PrimitiveComponent.SetLinearDamping` _cube 0.01)
      (`PrimitiveComponent.SetAngularDamping` _cube 0.0))))

(fn `UserConstructionScript`)